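; BP_AutoLaser is a laser trap that fires when a MyCharacter enters its Box trigger.
; Box overlap sets LaserReady and calls LaserStartSaphir, which spawns a one-tenth-scale BP_LaserEnemy at the Arrow and attaches it there.
; LaserReady resets after a short delay, but each new overlap also forces it true, bypassing that cooldown.
; Leaving the box calls SaphirNoHit on the character.
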(event `LaserStartSaphir`
  (bind _arrow (`self.Arrow`))
  (bind (_returnvalue_location _returnvalue_rotation _returnvalue_scale) (`KismetMathLibrary.BreakTransform` (`SceneComponent.K2_GetComponentToWorld` _arrow)))
  (if (`self.LaserReady`)
    (set `self.LaserReady` false)
    (bind _returnvalue (`|SpawnActorFromClass` "/Game/Core/WeaponsAndProjectiles/BP_LaserEnemy.BP_LaserEnemy_C" (`KismetMathLibrary.MakeTransform` _returnvalue_location _returnvalue_rotation (/ _returnvalue_scale 10)) "Undefined" "OverrideRootScale" null null))
    (`self.K2_AttachToComponent` _returnvalue _arrow "spine_004Socket" "SnapToTarget" "SnapToTarget" "SnapToTarget" true)
    (`KismetSystemLibrary.Delay` 0.5)
    (set `self.LaserReady` true)))

(event `self.Box.OnComponentBeginOverlap`
  (params (OverlappedComponent :type "PrimitiveComponent Object Reference") (OtherActor :type "Actor Object Reference") (OtherComp :type "PrimitiveComponent Object Reference") (OtherBodyIndex :type Integer) (bFromSweep :type Boolean) (SweepResult :type "HitResult Structure (by ref)"))
  (bind _asmy_character (cast `/Game/Core/MyCharacter` OtherActor))
  (set `self.As My Character` _asmy_character)
  (if true
    (set `self.LaserReady` true)
    (`self.LaserStartSaphir`)))

(event `self.Box.OnComponentEndOverlap`
  (params (OverlappedComponent :type "PrimitiveComponent Object Reference") (OtherActor :type "Actor Object Reference") (OtherComp :type "PrimitiveComponent Object Reference") (OtherBodyIndex :type Integer))
  (bind _asmy_character (cast `/Game/Core/MyCharacter` OtherActor))
  (`/Game/Core/MyCharacter.SaphirNoHit` _asmy_character))

(fn `UserConstructionScript`)