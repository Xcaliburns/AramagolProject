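; BP_PanneauSimple is a simple sign that shows a text message to the player.
; Overlapping its Box with a "Player"-tagged actor displays an interact prompt widget, and leaving removes both the prompt and any open dialogue.
; The Dialogue event toggles a WBP_Dialogue widget filled with the sign's Text variable; nothing in this graph calls it.
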(event `self.Box.OnComponentBeginOverlap`
  (params (OverlappedComponent :type "PrimitiveComponent Object Reference") (OtherActor :type "Actor Object Reference") (OtherComp :type "PrimitiveComponent Object Reference") (OtherBodyIndex :type Integer) (bFromSweep :type Boolean) (SweepResult :type "HitResult Structure (by ref)"))
  (if (`self.ActorHasTag` OtherActor "Player")
    (bind _returnvalue (`|CreateWidget` "/Game/Core/DialogueSystem/WBP_EtoInteract.WBP_EtoInteract_C" (`GameplayStatics.GetPlayerController` 0)))
    (bind _output_get (set `self.EToInteractWidget` _returnvalue))
    (`UserWidget.AddToViewport` _output_get 0)))

(event `self.Box.OnComponentEndOverlap`
  (params (OverlappedComponent :type "PrimitiveComponent Object Reference") (OtherActor :type "Actor Object Reference") (OtherComp :type "PrimitiveComponent Object Reference") (OtherBodyIndex :type Integer))
  (bind _dialoguewidget (`self.DialogueWidget`))
  (bind _etointeractwidget (`self.EToInteractWidget`))
  (if (`self.ActorHasTag` OtherActor "Player")
    (`/Engine/EditorBlueprintResources/StandardMacros.IsValid` _etointeractwidget
      (:`Is Valid`
        (`Widget.RemoveFromParent` _etointeractwidget))
      (:`Is Not Valid`
        _))
    (`/Engine/EditorBlueprintResources/StandardMacros.IsValid` _dialoguewidget
      (:`Is Valid`
        (`Widget.RemoveFromParent` _dialoguewidget :!label _label)
        (set `self.DialogueWidget` null)))))

(event `/Game/Core/DialogueSystem/BPI_Dialogue.Dialogue`
  (`/Engine/EditorBlueprintResources/StandardMacros.IsValid` (`self.DialogueWidget`)
    (:`Is Valid`
      (goto _label))
    (:`Is Not Valid`
      (bind _returnvalue (`|CreateWidget` "/Game/Core/DialogueSystem/WBP_Dialogue.WBP_Dialogue_C" (`GameplayStatics.GetPlayerController` 0)))
      (bind _output_get (set `self.DialogueWidget` _returnvalue))
      (`UserWidget.AddToViewport` _output_get 0)
      (set `/Game/Core/DialogueSystem/WBP_Dialogue.DialogueText` (`self.Text`) (`self.DialogueWidget`)))))

(fn `UserConstructionScript`)