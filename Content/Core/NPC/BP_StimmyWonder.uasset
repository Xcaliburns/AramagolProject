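; BP_StimmyWonder is an NPC that shows an interact prompt and gives dialogue based on which gem keys the player character holds.
; Its Box overlap caches the MyCharacter and shows the prompt widget; a Player-tagged actor leaving removes both prompt and dialogue.
; The Dialogue event toggles the dialogue widget, setting its text from the first true key flag in Diamant, Rubis, Emeraude, Saphir order.
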(event `self.Box.OnComponentBeginOverlap`
  (params (OverlappedComponent :type "PrimitiveComponent Object Reference") (OtherActor :type "Actor Object Reference") (OtherComp :type "PrimitiveComponent Object Reference") (OtherBodyIndex :type Integer) (bFromSweep :type Boolean) (SweepResult :type "HitResult Structure (by ref)"))
  (bind _asmy_character (cast `/Game/Core/MyCharacter` OtherActor))
  (set `self.As My Character` _asmy_character)
  (bind _returnvalue (`|CreateWidget` "/Game/Core/DialogueSystem/WBP_EtoInteract.WBP_EtoInteract_C" (`GameplayStatics.GetPlayerController` 0)))
  (bind _output_get (set `self.EToInteractWidget` _returnvalue))
  (`UserWidget.AddToViewport` _output_get 0))

(event `self.Box.OnComponentEndOverlap`
  (params (OverlappedComponent :type "PrimitiveComponent Object Reference") (OtherActor :type "Actor Object Reference") (OtherComp :type "PrimitiveComponent Object Reference") (OtherBodyIndex :type Integer))
  (bind _dialoguewidget (`self.DialogueWidget`))
  (bind _etointeractwidget (`self.EToInteractWidget`))
  (if (`self.ActorHasTag` OtherActor "Player")
    (`/Engine/EditorBlueprintResources/StandardMacros.IsValid` _etointeractwidget
      (:`Is Valid`
        (`Widget.RemoveFromParent` _etointeractwidget))
      (:`Is Not Valid`
        _))
    (`/Engine/EditorBlueprintResources/StandardMacros.IsValid` _dialoguewidget
      (:`Is Valid`
        (`Widget.RemoveFromParent` _dialoguewidget :!label _label)
        (set `self.DialogueWidget` null)))))

(event `/Game/Core/DialogueSystem/BPI_Dialogue.Dialogue`
  (bind _dialoguewidget (`self.DialogueWidget`))
  (bind _as_my_character (`self.As My Character`))
  (`/Engine/EditorBlueprintResources/StandardMacros.IsValid` (`self.DialogueWidget`)
    (:`Is Valid`
      (goto _label))
    (:`Is Not Valid`
      (bind _returnvalue (`|CreateWidget` "/Game/Core/DialogueSystem/WBP_Dialogue.WBP_Dialogue_C" (`GameplayStatics.GetPlayerController` 0)))
      (bind _output_get (set `self.DialogueWidget` _returnvalue))
      (`UserWidget.AddToViewport` _output_get 0)
      (if (`/Game/Core/MyCharacter.CleDiamant` _as_my_character)
        (set `/Game/Core/DialogueSystem/WBP_Dialogue.DialogueText` (`self.TextDiamant`) _dialoguewidget)
        (elif (`/Game/Core/MyCharacter.CleRubis` _as_my_character)
          (set `/Game/Core/DialogueSystem/WBP_Dialogue.DialogueText` (`self.TextRubis`) _dialoguewidget)
          (elif (`/Game/Core/MyCharacter.CleEmeraude` _as_my_character)
            (set `/Game/Core/DialogueSystem/WBP_Dialogue.DialogueText` (`self.TextEmeraude`) _dialoguewidget)
            (elif (`/Game/Core/MyCharacter.CleSaphir` _as_my_character)
              (set `/Game/Core/DialogueSystem/WBP_Dialogue.DialogueText` (`self.TextSaphir`) _dialoguewidget))))))))

(fn `UserConstructionScript`)