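; Laser enemy actor that fires a colored beam along its forward vector and notifies the player character when the beam hits it.
; Each Tick, a Visibility line trace places the beam end and impact effect, shortening the reach on a hit and regrowing it over time up to a cap.
; Two cross-resetting DoOnce gates send SaphirHited and SaphirNoHit only on changes between player and other hit actors.
; An older tag-based damage path is left disconnected.
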(event `self.ReceiveBeginPlay`
  (`FXSystemComponent.SetColorParameter` (`self.Laser`) "CustomColor" (`self.LaserColor`))
  (`FXSystemComponent.SetColorParameter` (`self.LaserImpact`) "CustomColor" (`self.LaserColor`)))

(event `self.ReceiveTick`
  (params (DeltaSeconds :type "Float (single-precision)"))
  (bind _returnvalue (`self.K2_GetActorLocation`))
  (bind _returnvalue_2 (+ _returnvalue (* (`self.GetActorForwardVector`) (`self.Distance`))))
  (`|ExecutionSequence`
    (:`then_0`
      (set `self.TraceEnd` _returnvalue_2)
      (bind _outhit (`KismetSystemLibrary.LineTraceSingle` _returnvalue _returnvalue_2 "TraceTypeQuery1"))
      (set `self.Out Hit Hit Actor` (`.HitActor` (`GameplayStatics.BreakHitResult` _outhit)))
      (set `self.Hit` (`GameplayStatics.BreakHitResult` _outhit))
      (`FXSystemComponent.SetVectorParameter` (`self.Laser`) "LaserEnd" (select `bool` (`self.Hit`) :`false` (`self.TraceEnd`) :`true` (`.Location` (`GameplayStatics.BreakHitResult` _outhit))))
      (`SceneComponent.K2_SetWorldLocation` (`self.LaserImpact`) (`.Location` (`GameplayStatics.BreakHitResult` _outhit)) false false)
      (if (`self.Hit`)
        (set `self.Distance` (`KismetMathLibrary.VSize` (- (`.Location` (`GameplayStatics.BreakHitResult` _outhit)) (`self.K2_GetActorLocation`))))
        (`/Engine/EditorBlueprintResources/StandardMacros.IsValid` (`self.Out Hit Hit Actor`)
          (:`Is Valid`
            ;[1 1 1] DegatsVersion19042022
            (bind _asmy_character (cast `/Game/Core/MyCharacter` (`GameplayStatics.GetPlayerCharacter` 0)))
            (bind _output_get (set `self.As My Character_0` _asmy_character))
            (if (== (`self.Out Hit Hit Actor`) _asmy_character)
              (`/Engine/EditorBlueprintResources/StandardMacros.DoOnce` false :!label _label
                (:`Completed`
                  (`/Game/Core/MyCharacter.SaphirHited` _output_get)
                  (goto _label_2 :!via `Reset`)))
              (else
                (`/Engine/EditorBlueprintResources/StandardMacros.DoOnce` false :!label _label_2
                  (:`Completed`
                    (`ActorComponent.Deactivate` (`self.LaserImpact`))
                    (`/Game/Core/MyCharacter.SaphirNoHit` _output_get)
                    (goto _label :!via `Reset`)))))))))
    (:`then_1`
      (if (< (`self.Distance`) 2000.0)
        (set `self.Distance` (+ (`self.Distance`) (* DeltaSeconds 2000.0)))))))

(fn `UserConstructionScript`)