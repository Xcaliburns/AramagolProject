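; BP_GunBasic is a basic automatic gun that fires projectiles repeatedly between start and stop calls.
; StartFiring passes a DoOnce, fires immediately, then runs a looping timer at a rate set by ProjectilesParSeconde.
; Each shot spawns BP_ProjectileBasic at ProjectileSpawnPoint, with an attached NS_GunBurst Niagara effect and a sound call.
; StopFiring clears the timer and resets the DoOnce.
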(event `FireProjectile`
  (bind _projectilespawnpoint (`self.ProjectileSpawnPoint`))
  ;[1 1 1] Spawn du projectile
  (if true
    ;[1 1 1] ProjectileBasic
    (`|SpawnActorFromClass` "/Game/Core/WeaponsAndProjectiles/BP_ProjectileBasic.BP_ProjectileBasic_C" (`SceneComponent.K2_GetComponentToWorld` (`self.ProjectileSpawnPoint`)) "Undefined" "OverrideRootScale" null null)
    (`NiagaraFunctionLibrary.SpawnSystemAttached` "/Game/Core/FX/LaserStart/NS_GunBurst.NS_GunBurst" _projectilespawnpoint "None" (0.0 0.0 0.0) (struct) "KeepRelativeOffset")
    (`GameplayStatics.PlaySoundAtLocation` null (`SceneComponent.K2_GetComponentLocation` _projectilespawnpoint) (struct) 1.0 1.0 0.0 null null null)))

(event `StartFiring`
  ;[1 1 1] tire des projectiles de maniere repetee
  (`/Engine/EditorBlueprintResources/StandardMacros.DoOnce` false :!label _label
    (:`Completed`
      (`self.FireProjectile`)
      (`KismetSystemLibrary.K2_SetTimer` null "FireProjectile" (/ 1.0 (`self.ProjectilesParSeconde`)) true))))

(event `StopFiring`
  ;[1 1 1] tire des projectiles de maniere repetee
  (`KismetSystemLibrary.K2_ClearTimer` null "FireProjectile")
  (goto _label :!via `Reset`))

(fn `UserConstructionScript`)