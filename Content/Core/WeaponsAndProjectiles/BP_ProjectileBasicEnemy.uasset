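; Basic enemy projectile that damages what it overlaps and explodes on impact.
; On actor overlap, targets implementing BPI_Damageable without the Enemy tag receive Damages through AffectHealthMessage.
; Sphere collision hits on actors without the Player tag skip the damage.
; Both paths share the same ending, spawning P_Explosion at the sphere and destroying the projectile.
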(event `self.ReceiveActorBeginOverlap`
  (params (OtherActor :type "Actor Object Reference"))
  ;[1 1 1] Fait des degats si actor possede bpi damageable
  (if (`KismetSystemLibrary.DoesImplementInterface` OtherActor "/Game/Core/BPInterfaces/BPI_Damageable.BPI_Damageable_C")
    (if (not (`self.ActorHasTag` OtherActor "Enemy"))
      (`KismetSystemLibrary.PrintString` "on est la")
      (message `/Game/Core/BPInterfaces/BPI_Damageable.AffectHealth` OtherActor (`self.Damages`))
      (`GameplayStatics.SpawnEmitterAtLocation` "/Game/StarterContent/Particles/P_Explosion.P_Explosion" (`SceneComponent.K2_GetComponentLocation` (`self.Spherecollision`)) :!label _label)
      (`self.K2_DestroyActor`))))

(event `self.Spherecollision.OnComponentHit`
  (params (HitComponent :type "PrimitiveComponent Object Reference") (OtherActor :type "Actor Object Reference") (OtherComp :type "PrimitiveComponent Object Reference") (NormalImpulse :type "Vector Structure") (Hit :type "HitResult Structure (by ref)"))
  ;[1 1 1] pour tout autre actor
  (if (not (`self.ActorHasTag` OtherActor "Player"))
    (goto _label)))

(fn `UserConstructionScript`)