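; BP_HeadHunter is a homing enemy projectile that chases the player, costs health on contact and self-destructs.
; A looping timer, started from the construction script with a randomized initial delay, retargets ProjectileMovement at the player's Shield component and turns Sphere1 toward the player.
; Overlapping MyCharacter sends negative health, then spawns a destroy effect and camera shake before removing the actor.
; Any AffectHealth event triggers the same destruction directly.
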(event `TimerFollowPlayer`
  (`KismetSystemLibrary.K2_SetTimerDelegate` (delegate `FollowPlayer`) 0.5 true 0.0 0.3))

(event `FollowPlayer`
  (bind _projectilemovement (`self.ProjectileMovement`))
  (bind _homingtarget (`self.FindHomingTarget`))
  (set `ProjectileMovementComponent.HomingTargetComponent` _homingtarget _projectilemovement)
  (set `ProjectileMovementComponent.bIsHomingProjectile` true _projectilemovement)
  (`SceneComponent.K2_SetWorldRotation` (`self.Sphere1`) (`KismetMathLibrary.MakeRotator` 0.0 (.pitch (`KismetMathLibrary.FindLookAtRotation` (`SceneComponent.K2_GetComponentLocation` (`self.Sphere1`)) (`self.K2_GetActorLocation` (`GameplayStatics.GetPlayerCharacter` 0)))) (.yaw (`KismetMathLibrary.FindLookAtRotation` (`SceneComponent.K2_GetComponentLocation` (`self.Sphere1`)) (`self.K2_GetActorLocation` (`GameplayStatics.GetPlayerCharacter` 0))))) false false))

(event `self.SphereCollision.OnComponentBeginOverlap`
  (params (OverlappedComponent :type "PrimitiveComponent Object Reference") (OtherActor :type "Actor Object Reference") (OtherComp :type "PrimitiveComponent Object Reference") (OtherBodyIndex :type Integer) (bFromSweep :type Boolean) (SweepResult :type "HitResult Structure (by ref)"))
  (bind _asmy_character (cast `/Game/Core/MyCharacter` OtherActor))
  (message `/Game/Core/BPInterfaces/BPI_Damageable.AffectHealth` _asmy_character -5.0)
  (`NiagaraFunctionLibrary.SpawnSystemAtLocation` "/Game/Core/FX/destroyedEnemy/NS_Destroy.NS_Destroy" (`SceneComponent.K2_GetComponentLocation` (`self.SphereCollision`)) :!label _label)
  (`GameplayStatics.PlayWorldCameraShake` "/Game/Core/Components/CS_CommonEnemyDestroyed.CS_CommonEnemyDestroyed_C" (`self.K2_GetActorLocation`) 0.0 2500.0)
  (`self.K2_DestroyActor`))

(event `/Game/Core/BPInterfaces/BPI_Damageable.AffectHealth`
  (params (Delta :type "Float (single-precision)"))
  (goto _label))

(fn `FindHomingTarget`
  (returns (HomingTarget :type "SceneComponent Object Reference"))
  (bind _returnvalue (`GameplayStatics.GetActorOfClass` "/Game/Core/MyCharacter.MyCharacter_C"))
  (bind _shield (`/Game/Core/MyCharacter.Shield` _returnvalue))
  (set `self.Distance` (`KismetMathLibrary.VSize` (- (`SceneComponent.K2_GetComponentLocation` _shield) (`self.K2_GetActorLocation`))))
  (bind _output_get (set `self.Shield` _shield))
  (return _output_get))

(fn `UserConstructionScript`
  (`self.TimerFollowPlayer`))