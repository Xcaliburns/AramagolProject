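; BP_LaserSaphir is the player's sapphire laser beam actor, damaging "Enemy"-tagged actors and messaging whatever it hits.
; Each tick, a visibility trace from the character's LaserSaphirOrigine along its forward vector sets the Niagara beam endpoints.
; DoOnce gates toggle the impact effect, while damage is a fixed per-tick amount, not delta-scaled.
; StopLaser deactivates the effects, halts damage, and runs a scale timeline before destroying the actor.
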(event `self.ReceiveTick`
  (params (DeltaSeconds :type "Float (single-precision)"))
  (bind _laserhit (`self.LaserHit`))
  ;[1 1 1] Gestion des tranform du laser et degats
  (bind _asmy_character (cast `/Game/Core/MyCharacter` (`GameplayStatics.GetPlayerCharacter` 0)))
  (bind _output_get (set `self.As My Character` _asmy_character))
  (bind _returnvalue (`SceneComponent.K2_GetComponentLocation` (`/Game/Core/MyCharacter.LaserSaphirOrigine` _asmy_character)))
  (`FXSystemComponent.SetVectorParameter` (`self.Laser`) "User.BeamStart" _returnvalue)
  (bind _outhit (`KismetSystemLibrary.LineTraceSingle` _returnvalue (+ _returnvalue (* (`SceneComponent.GetForwardVector` (`Actor.RootComponent` _output_get)) (`self.LaserLongueurMax`))) "TraceTypeQuery1"))
  (bind (_bblockinghit _binitialoverlap _time _distance _location _impactpoint _normal _impactnormal _physmat _hitactor _hitcomponent _hitbonename _hititem _elementindex _faceindex _tracestart _traceend) (`GameplayStatics.BreakHitResult` _outhit))
  (bind _returnvalue_2 (`KismetSystemLibrary.IsValid` _hitcomponent))
  (`FXSystemComponent.SetVectorParameter` (`self.Laser`) "User.BeamEnd" (`KismetMathLibrary.SelectVector` _impactpoint _traceend _returnvalue_2))
  (`|ExecutionSequence`
    (:`then_0`
      ;;[1 1 1] LaserHitActive/Desactive
      (if _returnvalue_2
        (`|ExecutionSequence`
          (:`then_0`
            (`FXSystemComponent.SetVectorParameter` _laserhit "User.HitLocation" _impactpoint)
            (`/Engine/EditorBlueprintResources/StandardMacros.DoOnce` false :!label _label
              (:`Completed`
                (if (not (`self.LaserHitEnd`))
                  (`ActorComponent.Activate` (`self.LaserHit`) false)))))
          (:`then_1`
            (goto _label_2 :!via `Reset`)))
        (else
          (`/Engine/EditorBlueprintResources/StandardMacros.DoOnce` false :!label _label_2
            (:`Completed`
              (message `/Game/Core/BPInterfaces/BPI_SaphirStop.SaphirStop` _hitactor)
              (`ActorComponent.Deactivate` _laserhit)
              (goto _label :!via `Reset`))))))
    (:`then_1`
      ;;[1 1 1] Degats provoqués
      (`/Engine/EditorBlueprintResources/StandardMacros.IsValid` _hitactor
        (:`Is Valid`
          (if (`self.ActorHasTag` _hitactor "Enemy")
            (if (not (`self.LaserHitEnd`))
              (message `/Game/Core/BPInterfaces/BPI_Damageable.AffectHealth` _hitactor -0.58))))))
    (:`then_2`
      (message `/Game/Core/BPInterfaces/BPI_SaphirInteract.SaphirInteraction` _hitactor 0.0 null))))

(event `StopLaser`
  (`/Engine/EditorBlueprintResources/StandardMacros.DoOnce` false
    (:`Completed`
      ;[1 1 1] arrete du laser
      (`ActorComponent.Deactivate` (`self.Laser`))
      (`ActorComponent.Deactivate` (`self.LaserFire`))
      (set `self.LaserHitEnd` true)
      (`ActorComponent.Deactivate` (`self.LaserHit`))
      (bind (_direction _scale) (`Timeline|StopEffect` :!via `PlayFromStart`)
        (:`Update`
          (`FXSystemComponent.SetFloatParameter` (`self.Laser`) "User.Scale" _scale))
        (:`Finished`
          (`self.K2_DestroyActor`))))))

(fn `UserConstructionScript`)