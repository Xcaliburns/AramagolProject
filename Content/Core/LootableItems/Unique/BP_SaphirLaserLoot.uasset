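; Unique loot pickup that gives the Saphir laser weapon to an overlapping MyCharacter, setting its weapon number and energy values.
; On pickup it records its object name in MyGameInstance and destroys itself; BeginPlay checks that record after a delay to remove already-collected copies.
; It also shows a WBP_SaphirWeapon widget, but the timed removal follows DestroyActor in the sequence, so it relies on a destroyed actor.
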(event `self.StaticMesh.OnComponentBeginOverlap`
  (params (OverlappedComponent :type "PrimitiveComponent Object Reference") (OtherActor :type "Actor Object Reference") (OtherComp :type "PrimitiveComponent Object Reference") (OtherBodyIndex :type Integer) (bFromSweep :type Boolean) (SweepResult :type "HitResult Structure (by ref)"))
  (bind _asmy_character (cast `/Game/Core/MyCharacter` OtherActor))
  (`|ExecutionSequence`
    (:`then_0`
      (set `/Game/Core/MyCharacter.WeaponNumber` 1 _asmy_character)
      (set `/Game/Core/MyCharacter.SaphirEnergy` 10.0 _asmy_character)
      (set `/Game/Core/MyCharacter.SaphirEnergyMax` 50.0 _asmy_character)
      (`self.PickUp`)
      (`KismetSystemLibrary.PrintString` (`KismetSystemLibrary.GetObjectName` self))
      (`self.K2_DestroyActor`))
    (:`then_1`
      (bind _returnvalue (`|CreateWidget` "/Game/Core/WBP/WBP_SaphirWeapon.WBP_SaphirWeapon_C"))
      (`UserWidget.AddToViewport` _returnvalue 0)
      (`KismetSystemLibrary.Delay` 5.0)
      (`Widget.RemoveFromParent` _returnvalue))))

(event `self.ReceiveBeginPlay`
  (`KismetSystemLibrary.Delay` 5.0)
  (bind _asmy_game_instance (cast `/Game/Core/MyGameInstance` (`GameplayStatics.GetGameInstance`)))
  (set `self.As My Game Instance` _asmy_game_instance)
  (bind _destroyedalready (`/Game/Core/MyGameInstance.CheckIfAlreadyDestroyed` _asmy_game_instance (`KismetStringLibrary.Conv_StringToName` (`KismetSystemLibrary.GetObjectName` self))))
  (if _destroyedalready
    (`self.K2_DestroyActor`)))

(event `PickUp`
  (bind _asmy_game_instance (cast `/Game/Core/MyGameInstance` (`GameplayStatics.GetGameInstance`)))
  (`/Game/Core/MyGameInstance.DestroyItem` _asmy_game_instance (`KismetStringLibrary.Conv_StringToName` (`KismetSystemLibrary.GetObjectName` self))))

(fn `UserConstructionScript`)