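; BP_CLefDeSaphir is a unique sapphire key pickup that the player collects by touching it.
; When MyCharacter overlaps the static mesh, it sets CleSaphir on the character, records its object name through MyGameInstance's DestroyItem, prints debug text and destroys itself.
; One second after BeginPlay, it asks the GameInstance whether that name was already destroyed and removes itself if so, so collected keys stay gone.
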(event `self.StaticMesh.OnComponentBeginOverlap`
  (params (OverlappedComponent :type "PrimitiveComponent Object Reference") (OtherActor :type "Actor Object Reference") (OtherComp :type "PrimitiveComponent Object Reference") (OtherBodyIndex :type Integer) (bFromSweep :type Boolean) (SweepResult :type "HitResult Structure (by ref)"))
  (bind _asmy_character (cast `/Game/Core/MyCharacter` OtherActor))
  (set `/Game/Core/MyCharacter.CleSaphir` true _asmy_character)
  (`self.PickUp`)
  (`KismetSystemLibrary.PrintString` (`KismetSystemLibrary.GetObjectName` self))
  (`KismetSystemLibrary.PrintString` "CleDeSaphirOk")
  (`self.K2_DestroyActor`))

(event `self.ReceiveBeginPlay`
  (`KismetSystemLibrary.Delay` 1.0)
  (bind _asmy_game_instance (cast `/Game/Core/MyGameInstance` (`GameplayStatics.GetGameInstance`)))
  (set `self.As My Game Instance` _asmy_game_instance)
  (bind _destroyedalready (`/Game/Core/MyGameInstance.CheckIfAlreadyDestroyed` _asmy_game_instance (`KismetStringLibrary.Conv_StringToName` (`KismetSystemLibrary.GetObjectName` self))))
  (if _destroyedalready
    (`self.K2_DestroyActor`)))

(event `PickUp`
  (bind _asmy_game_instance (cast `/Game/Core/MyGameInstance` (`GameplayStatics.GetGameInstance`)))
  (`/Game/Core/MyGameInstance.DestroyItem` _asmy_game_instance (`KismetStringLibrary.Conv_StringToName` (`KismetSystemLibrary.GetObjectName` self))))

(fn `UserConstructionScript`)