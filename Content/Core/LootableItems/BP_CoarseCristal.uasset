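; BP_CoarseCristal is a lootable pickup that adds coarse cristal to the player's character.
; When the player character overlaps its static mesh, it raises MyCharacter's CoarseCristal count by CoarseCristalAmount, clamped between zero and the character's maximum.
; It then spawns an emitter and a sound at its location and destroys itself, even if the count is already full.
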(event `self.StaticMesh.OnComponentBeginOverlap`
  (params (OverlappedComponent :type "PrimitiveComponent Object Reference") (OtherActor :type "Actor Object Reference") (OtherComp :type "PrimitiveComponent Object Reference") (OtherBodyIndex :type Integer) (bFromSweep :type Boolean) (SweepResult :type "HitResult Structure (by ref)"))
  (bind _returnvalue (`GameplayStatics.GetPlayerCharacter` 0))
  (bind _returnvalue_2 (`SceneComponent.K2_GetComponentLocation` (`self.DefaultSceneRoot`)))
  (if (== OtherActor _returnvalue)
    (bind _asmy_character (cast `/Game/Core/MyCharacter` _returnvalue))
    (set `/Game/Core/MyCharacter.CoarseCristal` (`KismetMathLibrary.Clamp` (+ (`/Game/Core/MyCharacter.CoarseCristal` _asmy_character) (`self.CoarseCristalAmount`)) 0 (`/Game/Core/MyCharacter.CoarseCristalMax` _asmy_character)) _asmy_character)
    (`GameplayStatics.SpawnEmitterAtLocation` null _returnvalue_2)
    (`GameplayStatics.SpawnSoundAtLocation` null _returnvalue_2 (struct) 1.0 1.0 0.0 null null)
    (`self.K2_DestroyActor`)))

(fn `UserConstructionScript`)