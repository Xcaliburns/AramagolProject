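; BP_Capsule is an interactable capsule actor in the starships set that shows the player dialogue text.
; Overlapping its collision box with a Player-tagged actor adds an "E to interact" widget, and leaving removes it along with any open dialogue.
; A Dialogue event toggles a dialogue widget, filling it with the actor's DialogueText variable when created.
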(event `self.CollisionBox.OnComponentBeginOverlap`
  (params (OverlappedComponent :type "PrimitiveComponent Object Reference") (OtherActor :type "Actor Object Reference") (OtherComp :type "PrimitiveComponent Object Reference") (OtherBodyIndex :type Integer) (bFromSweep :type Boolean) (SweepResult :type "HitResult Structure (by ref)"))
  (if (`self.ActorHasTag` OtherActor "Player")
    (bind _returnvalue (`|CreateWidget` "/Game/Core/DialogueSystem/WBP_EtoInteract.WBP_EtoInteract_C" (`GameplayStatics.GetPlayerController` 0)))
    (bind _output_get (set `self.EToInteract` _returnvalue))
    (`UserWidget.AddToViewport` _output_get 0)))

(event `self.CollisionBox.OnComponentEndOverlap`
  (params (OverlappedComponent :type "PrimitiveComponent Object Reference") (OtherActor :type "Actor Object Reference") (OtherComp :type "PrimitiveComponent Object Reference") (OtherBodyIndex :type Integer))
  (bind _etointeract (`self.EToInteract`))
  (bind _dailoguewidget (`self.DailogueWidget`))
  (if (`self.ActorHasTag` OtherActor "Player")
    (`/Engine/EditorBlueprintResources/StandardMacros.IsValid` _etointeract
      (:`Is Valid`
        (`Widget.RemoveFromParent` _etointeract))
      (:`Is Not Valid`
        _))
    (`/Engine/EditorBlueprintResources/StandardMacros.IsValid` _dailoguewidget
      (:`Is Valid`
        (`Widget.RemoveFromParent` _dailoguewidget :!label _label)
        (set `self.DailogueWidget` null)))))

(event `/Game/Core/DialogueSystem/BPI_Dialogue.Dialogue`
  (`/Engine/EditorBlueprintResources/StandardMacros.IsValid` (`self.DailogueWidget`)
    (:`Is Valid`
      (goto _label))
    (:`Is Not Valid`
      (bind _returnvalue (`|CreateWidget` "/Game/Core/DialogueSystem/WBP_Dialogue.WBP_Dialogue_C" (`GameplayStatics.GetPlayerController` 0)))
      (bind _output_get (set `self.DailogueWidget` _returnvalue))
      (`UserWidget.AddToViewport` _output_get 0)
      (set `/Game/Core/DialogueSystem/WBP_Dialogue.DialogueText` (`self.Dialogue Text`) (`self.DailogueWidget`)))))

(fn `UserConstructionScript`)