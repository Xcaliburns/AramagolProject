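; BP_regenHealth is a regeneration fountain that restores health to a MyCharacter standing inside its box volume.
; Box overlap stores the character and starts a looping timer that repeatedly adds EnergyRecoveryAmount to its Health, clamped to MaxHealth.
; When that character leaves the box, the timer is paused by the Regen function name.
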(event `RegenTimer`
  (`KismetSystemLibrary.K2_SetTimerDelegate` (delegate `Regen`) 0.2 true))

(event `Regen`
  (bind _as_my_character (`self.As My Character`))
  (set `/Game/Core/MyCharacter.Health` (`KismetMathLibrary.FClamp` (+ (`/Game/Core/MyCharacter.Health` _as_my_character) (`self.EnergyRecoveryAmount`)) 0.0 (`/Game/Core/MyCharacter.MaxHealth` _as_my_character)) _as_my_character))

(event `self.Box.OnComponentBeginOverlap`
  (params (OverlappedComponent :type "PrimitiveComponent Object Reference") (OtherActor :type "Actor Object Reference") (OtherComp :type "PrimitiveComponent Object Reference") (OtherBodyIndex :type Integer) (bFromSweep :type Boolean) (SweepResult :type "HitResult Structure (by ref)"))
  (bind _asmy_character (cast `/Game/Core/MyCharacter` OtherActor))
  (set `self.As My Character` _asmy_character)
  (`self.RegenTimer`))

(event `self.Box.OnComponentEndOverlap`
  (params (OverlappedComponent :type "PrimitiveComponent Object Reference") (OtherActor :type "Actor Object Reference") (OtherComp :type "PrimitiveComponent Object Reference") (OtherBodyIndex :type Integer))
  (if (== OtherActor (`self.As My Character`))
    (`KismetSystemLibrary.K2_PauseTimer` null "Regen")))

(fn `UserConstructionScript`)