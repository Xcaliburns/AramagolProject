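; Refinery regen fountain that converts the player's CoarseCristal into gem energy for the selected weapon.
; Box overlap caches MyCharacter and starts a looping timer, paused on exit.
; Each tick with crystals left runs the Saphir, Emerald or Ruby regen, then spends one crystal, even at full energy.
; Regen adds clamped energy or pauses the timer at max; Emerald's branch is hard-wired true, so it only pauses.
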(event `CoarseCristalPrice`
  (bind _as_my_character (`self.As My Character`))
  (set `/Game/Core/MyCharacter.CoarseCristal` (- (`/Game/Core/MyCharacter.CoarseCristal` _as_my_character) 1) _as_my_character))

(event `SaphirRegen`
  (bind _as_my_character (`self.As My Character`))
  (bind _saphirenergy (`/Game/Core/MyCharacter.SaphirEnergy` _as_my_character))
  (bind _saphirenergymax (`/Game/Core/MyCharacter.SaphirEnergyMax` _as_my_character))
  ;[1 1 1] SaphirRegen
  (if (== _saphirenergy _saphirenergymax)
    (`KismetSystemLibrary.K2_PauseTimerHandle` (`self.TimerHandle`))
    (elif (< _saphirenergy _saphirenergymax)
      (set `/Game/Core/MyCharacter.SaphirEnergy` (`KismetMathLibrary.FClamp` (+ _saphirenergy (`self.EnergyRecoveryAmount`)) 0.0 _saphirenergymax) _as_my_character))))

(event `EmeraldRegen`
  (bind _as_my_character (`self.As My Character`))
  (bind _emeraudeenergy (`/Game/Core/MyCharacter.EmeraudeEnergy` _as_my_character))
  (bind _emeraudeenergymax (`/Game/Core/MyCharacter.EmeraudeEnergyMax` _as_my_character))
  ;[1 1 1] EmeraldRegen
  (if true
    (`KismetSystemLibrary.K2_PauseTimerHandle` (`self.TimerHandle`))
    (elif (< _emeraudeenergy _emeraudeenergymax)
      (set `/Game/Core/MyCharacter.EmeraudeEnergy` (`KismetMathLibrary.FClamp` (+ _emeraudeenergy (`self.EnergyRecoveryAmount`)) 0.0 _emeraudeenergymax) _as_my_character))))

(event `RubyRegen`
  (bind _as_my_character (`self.As My Character`))
  (bind _rubisenergy (`/Game/Core/MyCharacter.RubisEnergy` _as_my_character))
  (bind _rubisenergymax (`/Game/Core/MyCharacter.RubisEnergyMax` _as_my_character))
  ;[1 1 1] RubyRegen
  (if (== _rubisenergy _rubisenergymax)
    (`KismetSystemLibrary.K2_PauseTimerHandle` (`self.TimerHandle`))
    (elif (< _rubisenergy _rubisenergymax)
      (set `/Game/Core/MyCharacter.RubisEnergy` (`KismetMathLibrary.FClamp` (+ _rubisenergy (`self.EnergyRecoveryAmount`)) 0.0 _rubisenergymax) _as_my_character))))

(event `RegenTimer`
  ;[1 1 1 1 47] RegenTimer
  (bind _returnvalue (`KismetSystemLibrary.K2_SetTimerDelegate` (delegate `Regen`) 0.2 true))
  (set `self.TimerHandle` _returnvalue))

(event `Regen`
  (bind _as_my_character (`self.As My Character`))
  ;[1 1 1 1 47] RegenTimer
  (if (> (`/Game/Core/MyCharacter.CoarseCristal` _as_my_character) 0)
    (switch `int` (`/Game/Core/MyCharacter.WeaponChoosed` _as_my_character)
      (:`1`
        (`self.SaphirRegen`))
      (:`2`
        (`self.EmeraldRegen`))
      (:`3`
        (`self.RubyRegen`)))
    (`self.CoarseCristalPrice`)))

(event `self.Box.OnComponentBeginOverlap`
  (params (OverlappedComponent :type "PrimitiveComponent Object Reference") (OtherActor :type "Actor Object Reference") (OtherComp :type "PrimitiveComponent Object Reference") (OtherBodyIndex :type Integer) (bFromSweep :type Boolean) (SweepResult :type "HitResult Structure (by ref)"))
  (bind _asmy_character (cast `/Game/Core/MyCharacter` OtherActor))
  (set `self.As My Character` _asmy_character)
  (`self.RegenTimer`))

(event `self.Box.OnComponentEndOverlap`
  (params (OverlappedComponent :type "PrimitiveComponent Object Reference") (OtherActor :type "Actor Object Reference") (OtherComp :type "PrimitiveComponent Object Reference") (OtherBodyIndex :type Integer))
  (if (== OtherActor (`self.As My Character`))
    (`KismetSystemLibrary.K2_PauseTimer` null "Regen")))

(fn `UserConstructionScript`)