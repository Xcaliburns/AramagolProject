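; BP_Tourelle4Shot is an enemy turret that spins and fires from four cannons while the player is within its detection sphere.
; Player overlap activates RotatingMovement and a looping timer at ShotSpeed shots per second, spawning BP_ProjectileBasicEnemy at each cannon; leaving stops both.
; The construction script applies RotationSpeed as yaw rate, but the node setting the sphere radius from DetectionSphere is unconnected.
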(event `4ShotTimer`
  (bind _returnvalue (`KismetSystemLibrary.K2_SetTimerDelegate` (delegate `4Shot`) (/ 1.0 (`self.ShotSpeed`)) true))
  (set `self.ShotTimer` _returnvalue))

(event `4Shot`
  (`|SpawnActorFromClass` "/Game/Core/WeaponsAndProjectiles/BP_ProjectileBasicEnemy.BP_ProjectileBasicEnemy_C" (`SceneComponent.K2_GetComponentToWorld` (`self.Canon1`)) "Undefined" "OverrideRootScale" null null)
  (`KismetSystemLibrary.PrintString` "Hello")
  (`|SpawnActorFromClass` "/Game/Core/WeaponsAndProjectiles/BP_ProjectileBasicEnemy.BP_ProjectileBasicEnemy_C" (`SceneComponent.K2_GetComponentToWorld` (`self.Canon2`)) "Undefined" "OverrideRootScale" null null)
  (`|SpawnActorFromClass` "/Game/Core/WeaponsAndProjectiles/BP_ProjectileBasicEnemy.BP_ProjectileBasicEnemy_C" (`SceneComponent.K2_GetComponentToWorld` (`self.Canon3`)) "Undefined" "OverrideRootScale" null null)
  (`|SpawnActorFromClass` "/Game/Core/WeaponsAndProjectiles/BP_ProjectileBasicEnemy.BP_ProjectileBasicEnemy_C" (`SceneComponent.K2_GetComponentToWorld` (`self.Canon4`)) "Undefined" "OverrideRootScale" null null))

(event `self.ReceiveBeginPlay`
  (`ActorComponent.SetActive` (`self.RotatingMovement`) false false))

(event `self.Sphere.OnComponentBeginOverlap`
  (params (OverlappedComponent :type "PrimitiveComponent Object Reference") (OtherActor :type "Actor Object Reference") (OtherComp :type "PrimitiveComponent Object Reference") (OtherBodyIndex :type Integer) (bFromSweep :type Boolean) (SweepResult :type "HitResult Structure (by ref)"))
  (if (`self.ActorHasTag` OtherActor "Player")
    (`ActorComponent.SetActive` (`self.RotatingMovement`) true false)
    (`self.4ShotTimer`)))

(event `self.Sphere.OnComponentEndOverlap`
  (params (OverlappedComponent :type "PrimitiveComponent Object Reference") (OtherActor :type "Actor Object Reference") (OtherComp :type "PrimitiveComponent Object Reference") (OtherBodyIndex :type Integer))
  (if (`self.ActorHasTag` OtherActor "Player")
    (`ActorComponent.SetActive` (`self.RotatingMovement`) false false)
    (`KismetSystemLibrary.K2_ClearAndInvalidateTimerHandle` (`self.ShotTimer`))))

(fn `UserConstructionScript`
  (set `RotatingMovementComponent.RotationRate` (`KismetMathLibrary.MakeRotator` 0.0 0.0 (`self.RotationSpeed`)) (`self.RotatingMovement`)))