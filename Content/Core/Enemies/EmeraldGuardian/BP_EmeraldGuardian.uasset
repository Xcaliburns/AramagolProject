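; Emerald Guardian enemy that, once triggered through Interactable, shows its own widget and starts an endless patrol over an array of target actors.
; At each stop it moves its capsule, then a timeline turns it toward the player while firing an attached laser, gated by a cooldown.
; Health changes flash the mesh material; at zero health it removes the widget, sends InverseMessage to its Interactor actors and destroys itself.
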(event `LaserStartEmerald`
  (bind _arrow1 (`self.Arrow1`))
  (bind (_returnvalue_location _returnvalue_rotation _returnvalue_scale) (`KismetMathLibrary.BreakTransform` (`SceneComponent.K2_GetComponentToWorld` _arrow1)))
  (if (`self.LaserReady`)
    (set `self.LaserReady` false)
    (bind _returnvalue (`|SpawnActorFromClass` "/Game/Core/WeaponsAndProjectiles/BP_LaserEnemy.BP_LaserEnemy_C" (`KismetMathLibrary.MakeTransform` _returnvalue_location _returnvalue_rotation (/ _returnvalue_scale 10)) "Undefined" "OverrideRootScale" null null))
    (`self.K2_AttachToComponent` _returnvalue _arrow1 "None" "SnapToTarget" "SnapToTarget" "SnapToTarget" true)
    (`KismetSystemLibrary.Delay` 2.3)
    (set `self.LaserReady` true)))

(event `/Game/Core/BPInterfaces/BPI_Interactable.Interactable`
  (params (Interactor :type "Actor Object Reference"))
  (set `self.LaserReady` true)
  (`self.Movement`)
  (bind _returnvalue (`|CreateWidget` "/Game/Core/WBP/BossesWidgets/WBP_EmeraldGuardian.WBP_EmeraldGuardian_C"))
  (bind _output_get (set `self.WBP_Ref` _returnvalue))
  (`UserWidget.AddToViewport` _output_get 0))

(event `/Game/Core/BPInterfaces/BPI_Damageable.AffectHealth`
  (params (Delta :type "Float (single-precision)"))
  (bind _mesh (`self.Mesh`))
  (bind _interactor (`self.Interactor`))
  (`KismetSystemLibrary.PrintString` "Hello")
  (bind _newhealth (`self.UpdateHealthPoints` Delta))
  (`KismetSystemLibrary.PrintString` (`KismetStringLibrary.Conv_DoubleToString` _newhealth))
  (if (`self.IsDead`)
    (`Widget.RemoveFromParent` (`self.WBP_Ref`))
    (for (_ _array_index) _interactor
      (message `/Game/Core/BPInterfaces/BPI_InverseInteract.Inverse` (`|GetArrayItem` _interactor _array_index) null))
    (`self.K2_DestroyActor`)
    (else
      (`PrimitiveComponent.SetMaterial` _mesh 1 "/Game/Core/Material/MI_Flash.MI_Flash")
      (`KismetSystemLibrary.Delay` 0.1)
      (`PrimitiveComponent.SetMaterial` _mesh 1 "/Game/Core/Starships/vert.vert"))))

(event `Movement`
  (bind _capsulecomponent (`self.CapsuleComponent`))
  (bind _target (`self.Target`))
  ;[1 1 1 1 47] Movement
  (bind (_arrayelement _arrayindex) (`/Game/Core/Macros/MacroLibrary.ForEachLoopWithDelay` _target 5.0)
    (:`LoopBody`
      (bind _output (`|GetArrayItem` _target _arrayindex))
      (`SceneComponent.K2_SetWorldRotation` (`self.CapsuleComponent`) (`KismetMathLibrary.MakeRotator` 0.0 (.pitch (`KismetMathLibrary.FindLookAtRotation` (`SceneComponent.K2_GetComponentLocation` (`self.CapsuleComponent`)) (`self.K2_GetActorLocation` _output))) (.yaw (`KismetMathLibrary.FindLookAtRotation` (`SceneComponent.K2_GetComponentLocation` (`self.CapsuleComponent`)) (`self.K2_GetActorLocation` _output)))) false false)
      (`KismetSystemLibrary.MoveComponentTo` (`self.CapsuleComponent`) (`self.K2_GetActorLocation` _output) (struct) false false 3.0 true)
      (`KismetSystemLibrary.Delay` 0.2)
      (bind (_direction _alpha) (`Timeline|Timeline_0` :!via `PlayFromStart`)
        (:`Update`
          (`SceneComponent.K2_SetWorldRotation` _capsulecomponent (`KismetMathLibrary.RLerp` (`SceneComponent.K2_GetComponentRotation` _capsulecomponent) (`KismetMathLibrary.MakeRotator` 0.0 (.pitch (`KismetMathLibrary.FindLookAtRotation` (`SceneComponent.K2_GetComponentLocation` (`self.CapsuleComponent`)) (`self.K2_GetActorLocation` (`GameplayStatics.GetPlayerCharacter` 0)))) (.yaw (`KismetMathLibrary.FindLookAtRotation` (`SceneComponent.K2_GetComponentLocation` (`self.CapsuleComponent`)) (`self.K2_GetActorLocation` (`GameplayStatics.GetPlayerCharacter` 0))))) _alpha) false false)
          (`self.LaserStartEmerald`))))
    (:`Completed`
      (`self.Movement`))))

(fn `UpdateHealthPoints`
  (params (Delta :type "Float (double-precision)"))
  (returns (NewHealth :type "Float (double-precision)"))
  (bind _output_get (set `self.Health` (+ (`self.Health`) Delta)))
  (`self.UpdateIsDead`)
  (return _output_get))

(fn `UpdateIsDead`
  (if (<= (`self.Health`) 0.0)
    (set `self.IsDead` true)
    (else
      (set `self.IsDead` false))))

(fn `UserConstructionScript`)