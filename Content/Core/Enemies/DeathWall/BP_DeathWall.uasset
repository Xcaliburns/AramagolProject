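; Death wall enemy that, once activated through Interactable, shows its widget, becomes damageable and slides its mesh toward the Objectif actor's location.
; Box overlap starts a looping timer that damages MyCharacter, paused when the player leaves.
; Each hit removes health and briefly flashes the wall and weakness meshes through a material swap.
; Death removes the widget, plays camera shake and destruction effects, sends InverseMessage to linked Interactors, then destroys the actor.
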(event `/Game/Core/BPInterfaces/BPI_Interactable.Interactable`
  (params (Interactor :type "Actor Object Reference"))
  (bind _returnvalue (`|CreateWidget` "/Game/Core/WBP/BossesWidgets/WBP_DeathWall.WBP_DeathWall_C"))
  (bind _output_get (set `self.WidgetRef` _returnvalue))
  (`UserWidget.AddToViewport` _output_get 0)
  (set `self.Damageable` true)
  (`KismetSystemLibrary.MoveComponentTo` (`self.StaticMeshComponent`) (`self.K2_GetActorLocation` (`self.Objectif`)) (struct) false false (`self.Over Time`)))

(event `TimerDamage`
  (bind _returnvalue (`KismetSystemLibrary.K2_SetTimerDelegate` (delegate `Damages`) 0.5 true))
  (set `self.TimerDamageHandle` _returnvalue))

(event `Damages`
  (`/Game/Core/MyCharacter.AffectHealth` (`self.As My Character`) -25.0))

(event `self.Box.OnComponentBeginOverlap`
  (params (OverlappedComponent :type "PrimitiveComponent Object Reference") (OtherActor :type "Actor Object Reference") (OtherComp :type "PrimitiveComponent Object Reference") (OtherBodyIndex :type Integer) (bFromSweep :type Boolean) (SweepResult :type "HitResult Structure (by ref)"))
  (bind _asmy_character (cast `/Game/Core/MyCharacter` OtherActor))
  (set `self.As My Character` _asmy_character)
  (`self.TimerDamage`))

(event `self.Box.OnComponentEndOverlap`
  (params (OverlappedComponent :type "PrimitiveComponent Object Reference") (OtherActor :type "Actor Object Reference") (OtherComp :type "PrimitiveComponent Object Reference") (OtherBodyIndex :type Integer))
  (if (`self.ActorHasTag` OtherActor "Player")
    (`KismetSystemLibrary.K2_PauseTimerHandle` (`self.TimerDamageHandle`))))

(event `/Game/Core/BPInterfaces/BPI_Damageable.AffectHealth`
  (params (Delta :type "Float (single-precision)"))
  (bind _interactor (`self.Interactor`))
  (bind _staticmeshcomponent (`self.StaticMeshComponent`))
  (if (`self.Damageable`)
    (bind _newhealth (`self.UpdateHealthPoints` -1.0))
    (`KismetSystemLibrary.PrintString` (`KismetStringLibrary.Conv_DoubleToString` _newhealth) true true (struct :`G` 0.66 :`B` 1.0 :`A` 1.0) _newhealth)
    (if (`self.IsDead`)
      (`Widget.RemoveFromParent` (`self.WidgetRef`))
      (`GameplayStatics.PlayWorldCameraShake` "/Game/Core/Components/CS_CommonEnemyDestroyed.CS_CommonEnemyDestroyed_C" (`self.K2_GetActorLocation`) 0.0 2500.0)
      (`NiagaraFunctionLibrary.SpawnSystemAtLocation` "/Game/Core/FX/destroyedEnemy/NS_Destroy.NS_Destroy")
      (for (_ _array_index) _interactor
        (message `/Game/Core/BPInterfaces/BPI_InverseInteract.Inverse` (`|GetArrayItem` _interactor _array_index) null))
      (`self.K2_DestroyActor`)
      (else
        (`PrimitiveComponent.SetMaterial` _staticmeshcomponent 0 "/Game/Core/Material/MI_Flash.MI_Flash")
        (`PrimitiveComponent.SetMaterial` (`self.DeathWall_DeathWall`) 0 "/Game/Core/Material/MI_Flash.MI_Flash")
        (`PrimitiveComponent.SetMaterial` (`self.DeathWall_DeathWallWeakness`) 0 "/Game/Core/Material/MI_Flash.MI_Flash")
        (`PrimitiveComponent.SetMaterial` (`self.DeathwallWeakness3`) 0 "/Game/Core/Material/MI_Flash.MI_Flash")
        (`PrimitiveComponent.SetMaterial` (`self.DeathWall_DeathWallWeakness1`) 0 "/Game/Core/Material/MI_Flash.MI_Flash")
        (`KismetSystemLibrary.Delay` 0.1)
        (`PrimitiveComponent.SetMaterial` _staticmeshcomponent 0 "/Engine/BasicShapes/BasicShapeMaterial.BasicShapeMaterial")
        (`PrimitiveComponent.SetMaterial` (`self.DeathWall_DeathWall`) 0 "/Engine/BasicShapes/BasicShapeMaterial.BasicShapeMaterial")
        (`PrimitiveComponent.SetMaterial` (`self.DeathWall_DeathWallWeakness`) 0 "/Engine/BasicShapes/BasicShapeMaterial.BasicShapeMaterial")
        (`PrimitiveComponent.SetMaterial` (`self.DeathwallWeakness3`) 0 "/Engine/BasicShapes/BasicShapeMaterial.BasicShapeMaterial")
        (`PrimitiveComponent.SetMaterial` (`self.DeathWall_DeathWallWeakness1`) 0 "/Engine/BasicShapes/BasicShapeMaterial.BasicShapeMaterial")))))

(fn `UpdateHealthPoints`
  (params (Delta :type "Float (double-precision)" :default -1.0))
  (returns (NewHealth :type "Float (double-precision)"))
  (bind _output_get (set `self.Health` (+ (`self.Health`) Delta)))
  (`self.UpdateIsDead`)
  (return _output_get))

(fn `UpdateIsDead`
  (if (<= (`self.Health`) 0.0)
    (set `self.IsDead` true)
    (`KismetSystemLibrary.K2_PauseTimer` null "UpdateHealthPoints")
    (else
      (set `self.IsDead` false))))

(fn `UserConstructionScript`)