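; Boss combat truck that, once triggered via Interactable, shows its fight widget and drives along a referenced spline using a Timeline.
; Looping timers aim both cannons at the player and fire projectiles from two muzzle points.
; A Box overlap damages the player on entry, then repeatedly by timer.
; Hits flash the hull material; death removes the widget, drops a health item, calls InverseMessage on linked interactors and destroys the truck.
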(event `FollowSplinePath`
  (bind _timeline_0 (`self.Timeline_0`))
  (bind _spline (`/Game/Core/BPSplinePath.Spline` (`self.SplinePathRef`)))
  (bind _returnvalue (`KismetMathLibrary.Lerp` 0.0 (`SplineComponent.GetSplineLength` _spline) (`self.Alpha`)))
  ;[1 1 1] SplinePath
  (`TimelineComponent.SetPlayRate` _timeline_0 (/ 1.0 (`self.Duration`)))
  (`TimelineComponent.SetNewTime` _timeline_0 (`self.StartOffset`))
  (bind (_direction _alpha) (`Timeline|Timeline_0`)
    (:`Update`
      (set `self.Alpha` _alpha)
      (`self.K2_SetActorLocationAndRotation` (`SplineComponent.GetLocationAtDistanceAlongSpline` _spline _returnvalue "World") (`SplineComponent.GetRotationAtDistanceAlongSpline` _spline _returnvalue "World")))))

(event `ShotTimer`
  ;[1 1 1] Shot
  (`KismetSystemLibrary.K2_SetTimerDelegate` (delegate `Shot`) 0.3 true))

(event `Shot`
  ;[1 1 1] Shot
  (`|SpawnActorFromClass` "/Game/Core/WeaponsAndProjectiles/BP_ProjectileLent.BP_ProjectileLent_C" (`SceneComponent.K2_GetComponentToWorld` (`self.CanonShot`)) "Undefined" "OverrideRootScale" null null)
  (`|SpawnActorFromClass` "/Game/Core/WeaponsAndProjectiles/BP_ProjectileLent.BP_ProjectileLent_C" (`SceneComponent.K2_GetComponentToWorld` (`self.CanonShot1`)) "Undefined" "OverrideRootScale" null null))

(event `TurretFaceTimer`
  ;[1 1 1] Fait tourner la tourelle vers le joueur
  (`KismetSystemLibrary.K2_SetTimerDelegate` (delegate `TurretFaceToPlayer`) 0.1 true))

(event `TurretFaceToPlayer`
  ;[1 1 1] Fait tourner la tourelle vers le joueur
  (`SceneComponent.K2_SetWorldRotation` (`self.vehiculeCombatPourExport_Canon`) (`KismetMathLibrary.MakeRotator` 0.0 (.pitch (`KismetMathLibrary.FindLookAtRotation` (`SceneComponent.K2_GetComponentLocation` (`self.vehiculeCombatPourExport_Canon`)) (`self.K2_GetActorLocation` (`GameplayStatics.GetPlayerCharacter` 0)))) (.yaw (`KismetMathLibrary.FindLookAtRotation` (`SceneComponent.K2_GetComponentLocation` (`self.vehiculeCombatPourExport_Canon`)) (`self.K2_GetActorLocation` (`GameplayStatics.GetPlayerCharacter` 0))))) false false)
  (`SceneComponent.K2_SetWorldRotation` (`self.vehiculeCombatPourExport_Canon1`) (`KismetMathLibrary.MakeRotator` 0.0 (.pitch (`KismetMathLibrary.FindLookAtRotation` (`SceneComponent.K2_GetComponentLocation` (`self.vehiculeCombatPourExport_Canon1`)) (`self.K2_GetActorLocation` (`GameplayStatics.GetPlayerCharacter` 0)))) (.yaw (`KismetMathLibrary.FindLookAtRotation` (`SceneComponent.K2_GetComponentLocation` (`self.vehiculeCombatPourExport_Canon1`)) (`self.K2_GetActorLocation` (`GameplayStatics.GetPlayerCharacter` 0))))) false false))

(event `/Game/Core/BPInterfaces/BPI_Interactable.Interactable`
  (params (Interactor :type "Actor Object Reference"))
  (bind _returnvalue (`|CreateWidget` "/Game/Core/WBP/BossesWidgets/WBP_FightTruck.WBP_FightTruck_C"))
  (bind _output_get (set `self.WidgetRef` _returnvalue))
  (`UserWidget.AddToViewport` _output_get 0)
  (`self.TurretFaceTimer`)
  (`self.ShotTimer`)
  (`self.FollowSplinePath`))

(event `self.Box.OnComponentBeginOverlap`
  (params (OverlappedComponent :type "PrimitiveComponent Object Reference") (OtherActor :type "Actor Object Reference") (OtherComp :type "PrimitiveComponent Object Reference") (OtherBodyIndex :type Integer) (bFromSweep :type Boolean) (SweepResult :type "HitResult Structure (by ref)"))
  ;[1 1 1 1 100] Gestion des degats au joueur
  ;;[1 1 1] Degats repetesAuJoueur
  (set `self.PlayerInRange` true)
  (bind _asmy_character (cast `/Game/Core/MyCharacter` OtherActor))
  (bind _output_get (set `self.As My Character` _asmy_character))
  (`/Engine/EditorBlueprintResources/StandardMacros.IsValid` _output_get
    (:`Is Valid`
      (`/Game/Core/MyCharacter.AffectHealth` (`self.DamageAmount`))
      (bind _returnvalue (`KismetSystemLibrary.K2_SetTimerDelegate` (delegate `DamageHero`) (/ 1.0 (`self.AttackPerSecond`)) true))
      (set `self.Timer` _returnvalue))
    (:`Is Not Valid`
      (set `self.PlayerInRange` false))))

(event `DamageHero`
  (bind _as_my_character (`self.As My Character`))
  ;[1 1 1 1 100] Gestion des degats au joueur
  ;;[1 1 1] Degats repetesAuJoueur
  ;;;[1 1 1] DegatsAuJoueur
  (if (`self.PlayerInRange`)
    (`/Engine/EditorBlueprintResources/StandardMacros.IsValid` _as_my_character
      (:`Is Valid`
        (`/Game/Core/BPInterfaces/BPI_Damageable.AffectHealth` _as_my_character (`self.DamageAmount`))))))

(event `self.Box.OnComponentEndOverlap`
  (params (OverlappedComponent :type "PrimitiveComponent Object Reference") (OtherActor :type "Actor Object Reference") (OtherComp :type "PrimitiveComponent Object Reference") (OtherBodyIndex :type Integer))
  ;[1 1 1 1 100] Gestion des degats au joueur
  ;;[1 1 1] Arret des degats au joueur
  (if (== OtherActor (`self.As My Character`))
    (`|ExecutionSequence`
      (:`then_0`
        (set `self.PlayerInRange` false)
        (`KismetSystemLibrary.K2_ClearAndInvalidateTimerHandle` (`self.Timer`))))))

(event `/Game/Core/BPInterfaces/BPI_Damageable.AffectHealth`
  (params (Delta :type "Float (single-precision)"))
  (bind _interactor (`self.Interactor`))
  (bind _vehiculecombatpourexport_mainstructure (`self.vehiculeCombatPourExport_MainStructure`))
  (`PrimitiveComponent.SetMaterial` _vehiculecombatpourexport_mainstructure 0 "/Game/Core/Material/MI_Flash.MI_Flash")
  (`KismetSystemLibrary.Delay` 0.1)
  (`PrimitiveComponent.SetMaterial` _vehiculecombatpourexport_mainstructure 0 "/Game/Core/Enemies/stitcher/noir.noir")
  (bind _newhealth (`self.UpdateHealthPoints` Delta))
  (`KismetSystemLibrary.PrintString` (`KismetStringLibrary.Conv_DoubleToString` _newhealth))
  (if (`self.IsDead`)
    (`Widget.RemoveFromParent` (`self.WidgetRef`))
    (`|SpawnActorFromClass` "/Game/Core/LootableItems/BP_HealthItem.BP_HealthItem_C" (`KismetMathLibrary.Conv_VectorToTransform` (`SceneComponent.K2_GetComponentLocation` (`self.vehiculeCombatPourExport_MainStructure`))) "Undefined" "OverrideRootScale" null null)
    (for (_ _array_index) _interactor
      (message `/Game/Core/BPInterfaces/BPI_InverseInteract.Inverse` (`|GetArrayItem` _interactor _array_index) null))
    (`self.K2_DestroyActor`)))

(fn `UpdateHealthPoints`
  (params (Delta :type "Float (double-precision)"))
  (returns (NewHealth :type "Float (double-precision)"))
  (bind _output_get (set `self.Health` (+ (`self.Health`) Delta)))
  (`self.UpdateIsDead`)
  (return _output_get))

(fn `UpdateIsDead`
  (if (<= (`self.Health`) 0.0)
    (set `self.IsDead` true)
    (`KismetSystemLibrary.K2_PauseTimer` null "UpdateHealthPoints")
    (return)
    (else
      (set `self.IsDead` false))))

(fn `UserConstructionScript`)