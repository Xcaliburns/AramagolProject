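; BP_Tourelle1Shot is an enemy turret that rotates its cannon and fires when it spots the player.
; The player entering the detection sphere plays a timeline that yaws the Canon, and leaving stops it.
; Each player overlap with the Sight component spawns one BP_ProjectileBasicEnemy at CanonShot and prints a debug message.
; The construction script sets the sphere radius from the DetectionSphere variable.
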(event `MovementAlle`
  (bind (_direction _rotation) (`Timeline|TurretRotation` :!via `PlayFromStart` :!label _label)
    (:`Update`
      (`SceneComponent.K2_SetRelativeRotation` (`self.Canon`) (`KismetMathLibrary.MakeRotator` 0.0 0.0 _rotation) false false))))

(event `MovementStop`
  (goto _label :!via `Stop`))

(event `self.Sphere.OnComponentBeginOverlap`
  (params (OverlappedComponent :type "PrimitiveComponent Object Reference") (OtherActor :type "Actor Object Reference") (OtherComp :type "PrimitiveComponent Object Reference") (OtherBodyIndex :type Integer) (bFromSweep :type Boolean) (SweepResult :type "HitResult Structure (by ref)"))
  (if (`self.ActorHasTag` OtherActor "Player")
    (`self.MovementAlle`)))

(event `self.Sphere.OnComponentEndOverlap`
  (params (OverlappedComponent :type "PrimitiveComponent Object Reference") (OtherActor :type "Actor Object Reference") (OtherComp :type "PrimitiveComponent Object Reference") (OtherBodyIndex :type Integer))
  (if (`self.ActorHasTag` OtherActor "Player")
    (`self.MovementStop`)))

(event `self.Sight.OnComponentBeginOverlap`
  (params (OverlappedComponent :type "PrimitiveComponent Object Reference") (OtherActor :type "Actor Object Reference") (OtherComp :type "PrimitiveComponent Object Reference") (OtherBodyIndex :type Integer) (bFromSweep :type Boolean) (SweepResult :type "HitResult Structure (by ref)"))
  (if (`self.ActorHasTag` OtherActor "Player")
    (`KismetSystemLibrary.PrintString` "Je t ai vu")
    (`|SpawnActorFromClass` "/Game/Core/WeaponsAndProjectiles/BP_ProjectileBasicEnemy.BP_ProjectileBasicEnemy_C" (`SceneComponent.K2_GetComponentToWorld` (`self.CanonShot`)) "AlwaysSpawn" "OverrideRootScale" null null)))

(fn `UserConstructionScript`
  (`SphereComponent.SetSphereRadius` (`self.Sphere`) (`self.DetectionSphere`) true))