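; Final boss cannon: a destructible turret that tracks player 0 and fires basic enemy projectiles.
; Looping timers, started from the Construction Script, aim the mesh at the player and spawn projectiles from the Arrow transform.
; AffectHealth applies health deltas, briefly flashing the material while the cannon survives.
; On death it drops a health item, calls InverseMessage on each linked Interactor and destroys itself.
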(event `TurretFaceTimer`
  ;[1 1 1] Fait tourner la tourelle vers le joueur
  (`KismetSystemLibrary.K2_SetTimerDelegate` (delegate `TurretFaceToPlayer`) 0.1 true))

(event `TurretFaceToPlayer`
  ;[1 1 1] Fait tourner la tourelle vers le joueur
  (`SceneComponent.K2_SetWorldRotation` (`self.StaticMesh`) (`KismetMathLibrary.MakeRotator` 0.0 (.pitch (`KismetMathLibrary.FindLookAtRotation` (`SceneComponent.K2_GetComponentLocation` (`self.StaticMesh`)) (`self.K2_GetActorLocation` (`GameplayStatics.GetPlayerCharacter` 0)))) (.yaw (`KismetMathLibrary.FindLookAtRotation` (`SceneComponent.K2_GetComponentLocation` (`self.StaticMesh`)) (`self.K2_GetActorLocation` (`GameplayStatics.GetPlayerCharacter` 0))))) false false)
  (`SceneComponent.K2_SetWorldRotation` (`self.StaticMesh`) (`KismetMathLibrary.MakeRotator` 0.0 (.pitch (`KismetMathLibrary.FindLookAtRotation` (`SceneComponent.K2_GetComponentLocation` (`self.StaticMesh`)) (`self.K2_GetActorLocation` (`GameplayStatics.GetPlayerCharacter` 0)))) (.yaw (`KismetMathLibrary.FindLookAtRotation` (`SceneComponent.K2_GetComponentLocation` (`self.StaticMesh`)) (`self.K2_GetActorLocation` (`GameplayStatics.GetPlayerCharacter` 0))))) false false))

(event `StopSHotTimer`
  ;[1 1 1] Shot
  (`KismetSystemLibrary.K2_ClearAndInvalidateTimerHandle` (stale `ShotTimer` _returnvalue)))

(event `ShotTimer`
  ;[1 1 1] Shot
  (bind _returnvalue (`KismetSystemLibrary.K2_SetTimerDelegate` (delegate `Shot`) 1.0 true)))

(event `Shot`
  ;[1 1 1] Shot
  (`|SpawnActorFromClass` "/Game/Core/WeaponsAndProjectiles/BP_ProjectileBasicEnemy.BP_ProjectileBasicEnemy_C" (`SceneComponent.K2_GetComponentToWorld` (`self.Arrow`)) "Undefined" "OverrideRootScale" null null))

(event `/Game/Core/BPInterfaces/BPI_Damageable.AffectHealth`
  (params (Delta :type "Float (single-precision)"))
  (bind _interactor (`self.Interactor`))
  (bind _staticmesh (`self.StaticMesh`))
  (bind _newhealth (`self.UpdateHealthPoints` Delta))
  (`KismetSystemLibrary.PrintString` (`KismetStringLibrary.Conv_DoubleToString` _newhealth))
  (if (`self.Is dead`)
    (`|SpawnActorFromClass` "/Game/Core/LootableItems/BP_HealthItem.BP_HealthItem_C" (`KismetMathLibrary.Conv_VectorToTransform` (`SceneComponent.K2_GetComponentLocation` (`self.StaticMesh`))) "Undefined" "OverrideRootScale" null null)
    (for (_ _array_index) _interactor
      (message `/Game/Core/BPInterfaces/BPI_InverseInteract.Inverse` (`|GetArrayItem` _interactor _array_index) null))
    (`self.K2_DestroyActor`)
    (else
      (`PrimitiveComponent.SetMaterial` _staticmesh 0 "/Game/Core/Material/MI_Flash.MI_Flash")
      (`KismetSystemLibrary.Delay` 0.1)
      (`PrimitiveComponent.SetMaterial` _staticmesh 0 "/Game/Core/Enemies/FinalBoss/BlackMetal.BlackMetal"))))

(fn `UpdateHealthPoints`
  (params (Delta :type "Float (double-precision)"))
  (returns (NewHealth :type "Float (double-precision)"))
  (bind _output_get (set `self.Health` (+ (`self.Health`) Delta)))
  (`self.UpdateIsDead`)
  (return _output_get))

(fn `UpdateIsDead`
  (if (<= (`self.Health`) 0.0)
    (set `self.Is dead` true)
    (`KismetSystemLibrary.K2_PauseTimer` null "UpdateHealthPoints")
    (return)
    (else
      (set `self.Is dead` false))))

(fn `UserConstructionScript`
  (`self.ShotTimer`)
  (`self.TurretFaceTimer`))