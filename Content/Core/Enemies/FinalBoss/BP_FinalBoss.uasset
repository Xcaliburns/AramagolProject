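; Final boss turret that starts its fight on Interactable, showing the WBP_LastGuardian widget.
; Looping timers aim the turret at the player and spawn staggered BP_HeadHunter volleys from eight arrows.
; Health changes flash the turret and trigger one-time spawns: cannons below half health, more cannons plus three gem shields below a quarter.
; Death removes the widget, sends InverseMessage to Interactor entries, and destroys all HeadHunters and the boss.
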(event `ShotTimer`
  ;[1 1 1] Shot
  (`KismetSystemLibrary.K2_SetTimerDelegate` (delegate `Shot`) 5.0 true))

(event `Shot`
  ;[1 1 1] Shot
  (bind _arrayelement (`/Game/Core/Macros/MacroLibrary.ForEachLoopWithDelay` (`|MakeArray` (`self.Arrow`) (`self.Arrow1`) (`self.Arrow2`) (`self.Arrow3`) (`self.Arrow4`) (`self.Arrow5`) (`self.Arrow6`) (`self.Arrow7`)) 0.3)
    (:`LoopBody`
      (`|SpawnActorFromClass` "/Game/Core/WeaponsAndProjectiles/BP_HeadHunter.BP_HeadHunter_C" (`SceneComponent.K2_GetComponentToWorld` _arrayelement) "Undefined" "OverrideRootScale" null null))))

(event `/Game/Core/BPInterfaces/BPI_Damageable.AffectHealth`
  (params (Delta :type "Float (single-precision)"))
  (bind _tourelleprincipale (`self.TourellePrincipale`))
  (bind _interactor (`self.Interactor`))
  (bind _newhealth (`self.UpdateHealthPoints` Delta))
  (`KismetSystemLibrary.PrintString` (`KismetStringLibrary.Conv_DoubleToString` _newhealth))
  (if (`self.IsDead`)
    ;[1 1 1] Affect health
    (`Widget.RemoveFromParent` (`self.WBPRef`))
    (for (_ _array_index) _interactor
      (message `/Game/Core/BPInterfaces/BPI_InverseInteract.Inverse` (`|GetArrayItem` _interactor _array_index) null))
    (bind _outactors (`GameplayStatics.GetAllActorsOfClass` "/Game/Core/WeaponsAndProjectiles/BP_HeadHunter.BP_HeadHunter_C"))
    (for _array_element _outactors
      (`self.K2_DestroyActor` _array_element))
    (`self.K2_DestroyActor`)
    (else
      (`PrimitiveComponent.SetMaterial` _tourelleprincipale 0 "/Game/Core/Material/MI_Flash.MI_Flash")
      (`KismetSystemLibrary.Delay` 0.1)
      (`PrimitiveComponent.SetMaterial` _tourelleprincipale 0 "/Game/Core/Enemies/FinalBoss/Plastic.Plastic"))))

(event `SpawnCanons`
  ;[1 1 1] Spawn des canons sup
  (if (< (`self.HealthPoints`) (/ (`self.MaxHealthPoints`) 2.0))
    (`/Engine/EditorBlueprintResources/StandardMacros.DoOnce` false
      (:`Completed`
        (`|SpawnActorFromClass` "/Game/Core/Enemies/FinalBoss/BP_FinalBossCanon.BP_FinalBossCanon_C" (`SceneComponent.K2_GetComponentToWorld` (`self.Canon1`)) "Undefined" "OverrideRootScale" null null)
        (`|SpawnActorFromClass` "/Game/Core/Enemies/FinalBoss/BP_FinalBossCanon.BP_FinalBossCanon_C" (`SceneComponent.K2_GetComponentToWorld` (`self.Canon2`)) "Undefined" "OverrideRootScale" null null)))))

(event `SpawnCanons2`
  (if (< (`self.HealthPoints`) (/ (`self.MaxHealthPoints`) 4.0))
    (`/Engine/EditorBlueprintResources/StandardMacros.DoOnce` false
      (:`Completed`
        (`|SpawnActorFromClass` "/Game/Core/Enemies/FinalBoss/BP_FinalBossCanon.BP_FinalBossCanon_C" (`SceneComponent.K2_GetComponentToWorld` (`self.Canon3`)) "Undefined" "OverrideRootScale" null null)
        (`|SpawnActorFromClass` "/Game/Core/Enemies/FinalBoss/BP_FinalBossCanon.BP_FinalBossCanon_C" (`SceneComponent.K2_GetComponentToWorld` (`self.Canon4`)) "Undefined" "OverrideRootScale" null null)
        (`|SpawnActorFromClass` "/Game/Core/Enemies/FinalBoss/BP_ShieldSaphir.BP_ShieldSaphir_C" (`SceneComponent.K2_GetComponentToWorld` (`self.Shield`)) "Undefined" "OverrideRootScale" null null)
        (`|SpawnActorFromClass` "/Game/Core/Enemies/FinalBoss/BP_ShieldRuby.BP_ShieldRuby_C" (`SceneComponent.K2_GetComponentToWorld` (`self.Shield1`)) "Undefined" "OverrideRootScale" null null)
        (`|SpawnActorFromClass` "/Game/Core/Enemies/FinalBoss/BP_ShieldEmerald.BP_ShieldEmerald_C" (`SceneComponent.K2_GetComponentToWorld` (`self.Shield2`)) "Undefined" "OverrideRootScale" null null)))))

(event `TurretFaceTimer`
  ;[1 1 1] Fait tourner la tourelle vers le joueur
  (`KismetSystemLibrary.K2_SetTimerDelegate` (delegate `TurretFaceToPlayer`) 0.1 true))

(event `TurretFaceToPlayer`
  ;[1 1 1] Fait tourner la tourelle vers le joueur
  (`SceneComponent.K2_SetWorldRotation` (`self.TourellePrincipale`) (`KismetMathLibrary.MakeRotator` 0.0 (.pitch (`KismetMathLibrary.FindLookAtRotation` (`SceneComponent.K2_GetComponentLocation` (`self.TourellePrincipale`)) (`self.K2_GetActorLocation` (`GameplayStatics.GetPlayerCharacter` 0)))) (.yaw (`KismetMathLibrary.FindLookAtRotation` (`SceneComponent.K2_GetComponentLocation` (`self.TourellePrincipale`)) (`self.K2_GetActorLocation` (`GameplayStatics.GetPlayerCharacter` 0))))) false false))

(event `/Game/Core/BPInterfaces/BPI_Interactable.Interactable`
  (params (Interactor :type "Actor Object Reference"))
  ;[1 1 1] Fait tourner la tourelle vers le joueur
  (bind _returnvalue (`|CreateWidget` "/Game/Core/WBP/BossesWidgets/WBP_LastGuardian.WBP_LastGuardian_C"))
  (bind _output_get (set `self.WBPRef` _returnvalue))
  (`UserWidget.AddToViewport` _output_get 0)
  (`self.TurretFaceTimer`)
  (`self.ShotTimer`))

(fn `UpdateHealthPoints`
  (params (Delta :type "Float (double-precision)"))
  (returns (NewHealth :type "Float (double-precision)"))
  (bind _output_get (set `self.HealthPoints` (+ (`self.HealthPoints`) Delta)))
  (`self.UpdateIsDead`)
  (`self.SpawnCanons`)
  (`self.SpawnCanons2`)
  (return _output_get))

(fn `UpdateIsDead`
  (if (<= (`self.HealthPoints`) 0.0)
    (set `self.IsDead` true)
    (`KismetSystemLibrary.K2_PauseTimer` null "UpdateHealthPoints")
    (return)
    (else
      (set `self.IsDead` false))))

(fn `UserConstructionScript`)