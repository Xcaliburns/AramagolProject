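; BP_ShieldEmerald is a destructible emerald in the final boss content that loses health each time it is interacted with.
; EmeraudeInteraction briefly swaps the mesh to a flash material, restores a translucent one, then subtracts a health point.
; UpdateHealthPoints prints the new health and calls UpdateIsDead, which sets the death flag at zero or below.
; The actor is destroyed only on the next interaction after that flag is set.
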(event `/Game/Core/BPInterfaces/BPI_EmeraudeInteract.EmeraudeInteraction`
  (bind _staticmesh (`self.StaticMesh`))
  (if (`self.IsDead`)
    (`self.K2_DestroyActor`)
    (else
      (`PrimitiveComponent.SetMaterial` _staticmesh 0 "/Game/Core/Material/MI_Flash.MI_Flash")
      (`KismetSystemLibrary.Delay` 0.1)
      (`PrimitiveComponent.SetMaterial` _staticmesh 0 "/Game/Core/Material/TranslucentLaserPointerMaterialInst2.TranslucentLaserPointerMaterialInst2")
      (`self.UpdateHealthPoints` -1.0))))

(fn `UpdateHealthPoints`
  (params (Delta :type "Float (double-precision)"))
  (returns (NewHealth :type "Float (double-precision)"))
  (bind _output_get (set `self.Health` (+ (`self.Health`) Delta)))
  (`KismetSystemLibrary.PrintString` (`KismetStringLibrary.Conv_DoubleToString` _output_get))
  (`self.UpdateIsDead`)
  (return _output_get))

(fn `UpdateIsDead`
  (if (<= (`self.Health`) 0.0)
    (set `self.IsDead` true)
    (`KismetSystemLibrary.K2_PauseTimer` null "UpdateHealthPoints")
    (return)
    (else
      (set `self.IsDead` false))))

(fn `UserConstructionScript`)