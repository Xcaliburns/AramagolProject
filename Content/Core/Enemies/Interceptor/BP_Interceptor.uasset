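; Interceptor enemy that, once activated through Interactable, shows its widget and patrols a looping series of Target actors while attacking the player.
; At each stop a timeline turns it toward the player and calls Shot on every update, spawning BP_ProjectileLent from the main cannon.
; AffectHealth applies health changes and briefly flashes the material.
; On death it removes the widget, sends InverseMessage to its Interactor actors and destroys itself.
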(event `/Game/Core/BPInterfaces/BPI_Damageable.AffectHealth`
  (params (Delta :type "Float (single-precision)"))
  (bind _interceptor (`self.Interceptor`))
  (bind _interactor (`self.Interactor`))
  (bind _newhealth (`self.UpdateHealthPoints` Delta))
  (`KismetSystemLibrary.PrintString` (`KismetStringLibrary.Conv_DoubleToString` _newhealth))
  (if (`self.IsDead`)
    (`Widget.RemoveFromParent` (`self.WBP_Ref`))
    (for (_ _array_index) _interactor
      (message `/Game/Core/BPInterfaces/BPI_InverseInteract.Inverse` (`|GetArrayItem` _interactor _array_index) null))
    (`self.K2_DestroyActor`)
    (else
      (`PrimitiveComponent.SetMaterial` _interceptor 0 "/Game/Core/Material/MI_Flash.MI_Flash")
      (`KismetSystemLibrary.Delay` 0.1)
      (`PrimitiveComponent.SetMaterial` _interceptor 0 "/Game/untitled_category/DecoMeshes/MetallicWhite.MetallicWhite"))))

(event `Movement`
  (bind _interceptor (`self.Interceptor`))
  (bind _target (`self.Target`))
  ;[1 1 1 1 47] Movement
  (bind (_arrayelement _arrayindex) (`/Game/Core/Macros/MacroLibrary.ForEachLoopWithDelay` _target 5.0)
    (:`LoopBody`
      (bind _output (`|GetArrayItem` _target _arrayindex))
      (`SceneComponent.K2_SetWorldRotation` (`self.Interceptor`) (`KismetMathLibrary.MakeRotator` 0.0 (.pitch (`KismetMathLibrary.FindLookAtRotation` (`SceneComponent.K2_GetComponentLocation` (`self.Interceptor`)) (`self.K2_GetActorLocation` _output))) (.yaw (`KismetMathLibrary.FindLookAtRotation` (`SceneComponent.K2_GetComponentLocation` (`self.Interceptor`)) (`self.K2_GetActorLocation` _output)))) false false)
      (`KismetSystemLibrary.MoveComponentTo` (`self.Interceptor`) (`self.K2_GetActorLocation` _output) (struct) false false 3.0 true)
      (`KismetSystemLibrary.Delay` 0.2)
      (bind (_direction _alpha) (`Timeline|AlphaRotation` :!via `PlayFromStart`)
        (:`Update`
          (`SceneComponent.K2_SetWorldRotation` _interceptor (`KismetMathLibrary.RLerp` (`SceneComponent.K2_GetComponentRotation` _interceptor) (`KismetMathLibrary.MakeRotator` 0.0 (.pitch (`KismetMathLibrary.FindLookAtRotation` (`SceneComponent.K2_GetComponentLocation` (`self.Interceptor`)) (`self.K2_GetActorLocation` (`GameplayStatics.GetPlayerCharacter` 0)))) (.yaw (`KismetMathLibrary.FindLookAtRotation` (`SceneComponent.K2_GetComponentLocation` (`self.Interceptor`)) (`self.K2_GetActorLocation` (`GameplayStatics.GetPlayerCharacter` 0))))) _alpha) false false)
          (`self.Shot`))))
    (:`Completed`
      (`self.Movement`))))

(event `Shot`
  ;[1 1 1 1 50] Shot
  (for _ (range 6)
    (`KismetSystemLibrary.Delay` 0.01)
    (`|SpawnActorFromClass` "/Game/Core/WeaponsAndProjectiles/BP_ProjectileLent.BP_ProjectileLent_C" (`SceneComponent.K2_GetComponentToWorld` (`self.CanonPrincipal`)) "Undefined" "OverrideRootScale" null null)))

(event `/Game/Core/BPInterfaces/BPI_Interactable.Interactable`
  (params (Interactor :type "Actor Object Reference"))
  (bind _returnvalue (`|CreateWidget` "/Game/Core/WBP/BossesWidgets/WBP_Interceptor.WBP_Interceptor_C"))
  (bind _output_get (set `self.WBP_Ref` _returnvalue))
  (`UserWidget.AddToViewport` _output_get 0)
  (`self.Movement`))

(fn `UpdateHealthPoints`
  (params (Delta :type "Float (double-precision)"))
  (returns (NewHealth :type "Float (double-precision)"))
  (bind _output_get (set `self.Health` (+ (`self.Health`) Delta)))
  (`self.UpdateIsDead`)
  (return _output_get))

(fn `UpdateIsDead`
  (if (<= (`self.Health`) 0.0)
    (set `self.IsDead` true)
    (`KismetSystemLibrary.K2_PauseTimer` null "UpdateHealthPoints")
    (return)
    (else
      (set `self.IsDead` false))))

(fn `UserConstructionScript`)