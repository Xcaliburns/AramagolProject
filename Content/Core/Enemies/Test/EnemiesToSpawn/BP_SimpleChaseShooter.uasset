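; BP_SimpleChaseShooter is a test enemy that shoots projectiles, takes damage and drops loot on death.
; A looping timer destroys it when the player is too far away or invalid.
; EnemyShot spawns a projectile at Arrow1 after a short delay.
; AffectHealth updates health and triggers random heal and sapphire drops on death; separate gem damage functions also update health, with Emeraude ignoring its delta and adding one.
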(event `self.ReceiveBeginPlay`
  ;[1 1 1] detruit l'ennemi si le joueur est trop loin
  (bind _returnvalue (`KismetSystemLibrary.K2_SetTimerDelegate` (delegate `DestroyIfPlayerIstooFar`) 2.0 true))
  (set `self.Timer` _returnvalue))

(event `DestroyIfPlayerIstooFar`
  ;[1 1 1] detruit l'ennemi si le joueur est trop loin
  (bind _asmy_character (cast `/Game/Core/MyCharacter` (`GameplayStatics.GetPlayerCharacter` 0)))
  (`/Engine/EditorBlueprintResources/StandardMacros.IsValid` _asmy_character
    (:`Is Valid`
      (bind _returnvalue (`self.GetDistanceTo` _asmy_character self))
      (`KismetSystemLibrary.PrintString` (`KismetStringLibrary.Conv_DoubleToString` _returnvalue))
      (if (>= _returnvalue (`self.DistanceMaxFromPlayer`))
        (`KismetSystemLibrary.K2_ClearAndInvalidateTimerHandle` (`self.Timer`) :!label _label)
        (`self.K2_DestroyActor`)))
    (:`Is Not Valid`
      (goto _label))))

(event `EnemyShot`
  ;[1 1 1] Shot
  (`KismetSystemLibrary.Delay` 0.2)
  (`|SpawnActorFromClass` "/Game/Core/WeaponsAndProjectiles/BP_ProjectileBasicEnemy.BP_ProjectileBasicEnemy_C" (`SceneComponent.K2_GetComponentToWorld` (`self.Arrow1`)) "Undefined" "OverrideRootScale" null null))

(event `/Game/Core/BPInterfaces/BPI_Damageable.AffectHealth`
  (params (Delta :type "Float (single-precision)"))
  ;[1 1 1] Gestion des degats Self
  (bind _newhealth (`self.UpdateHealthPoints` Delta))
  (`KismetSystemLibrary.PrintString` (`KismetStringLibrary.Conv_DoubleToString` _newhealth))
  (if (`self.IsDead`)
    (if (<= (`self.LootHealFloat`) (`KismetMathLibrary.RandomFloatInRange` 0.0 100.0))
      (`|SpawnActorFromClass` "/Game/Core/LootableItems/BP_HealthItem.BP_HealthItem_C" (`KismetMathLibrary.Conv_VectorToTransform` (`SceneComponent.K2_GetComponentLocation` (`self.CapsuleComponent`))) "Undefined" "OverrideRootScale" null null))
    (if (<= (`self.LootSaphir`) (`KismetMathLibrary.RandomFloatInRange` 0.0 100.0))
      (`|SpawnActorFromClass` "/Game/Core/LootableItems/BP_SaphirItem.BP_SaphirItem_C" (`KismetMathLibrary.Conv_VectorToTransform` (`SceneComponent.K2_GetComponentLocation` (`self.CapsuleComponent`))) "Undefined" "OverrideRootScale" null null))
    (`self.K2_DestroyActor`)))

(fn `DiamantDamages`
  (params (DeltaDiamant :type "Float (double-precision)"))
  (returns (NewHealth :type "Float (double-precision)"))
  (bind _output_get (set `self.Health` (+ (`self.Health`) DeltaDiamant)))
  (`self.UpdateIsDead`)
  (return _output_get))

(fn `EmeraudeDamages`
  (params (DeltaEmeraude :type "Float (double-precision)" :default -1.0))
  (returns (NewHealth :type "Float (double-precision)"))
  (bind _output_get (set `self.Health` (+ (`self.Health`) 1.0)))
  (`self.UpdateIsDead`)
  (return _output_get))

(fn `RubisDamages`
  (params (DeltaRubis :type "Float (double-precision)" :default -1.0))
  (returns (NewHealth :type "Float (double-precision)"))
  (bind _output_get (set `self.Health` (+ (`self.Health`) DeltaRubis)))
  (`self.UpdateIsDead`)
  (return _output_get))

(fn `SaphirDamages`
  (params (DeltaSaphir :type "Float (double-precision)" :default 0.0))
  (returns (NewHealth :type "Float (double-precision)"))
  (bind _output_get (set `self.Health` (+ (`self.Health`) DeltaSaphir)))
  (`self.UpdateIsDead`)
  (return _output_get))

(fn `UpdateHealthPoints`
  (params (Delta :type "Float (double-precision)"))
  (returns (NewHealth :type "Float (double-precision)"))
  (bind _output_get (set `self.Health` (+ (`self.Health`) Delta)))
  (`self.UpdateIsDead`)
  (return _output_get))

(fn `UpdateIsDead`
  (if (<= (`self.Health`) 0.0)
    (set `self.IsDead` true)
    (`KismetSystemLibrary.K2_PauseTimer` null "UpdateHealthPoints")
    (else
      (set `self.IsDead` false))))

(fn `UserConstructionScript`)