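; Test enemy Blueprint for a Saphir chaser that damages the player, takes Saphir laser hits and despawns when too far away; no movement logic appears here.
; A looping timer checks distance, while box overlap deals immediate damage then starts a repeating damage timer, overwriting the same Timer handle.
; Laser overlaps on the capsule reduce Health; death rolls for heal and Saphir item drops, then destroys the actor.
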(event `self.ReceiveBeginPlay`
  ;[1 1 1] detruit l'ennemi si le joueur est trop loin
  (bind _returnvalue (`KismetSystemLibrary.K2_SetTimerDelegate` (delegate `DestroyIfPlayerIstooFar`) 2.0 true))
  (set `self.Timer` _returnvalue))

(event `DestroyIfPlayerIstooFar`
  ;[1 1 1] detruit l'ennemi si le joueur est trop loin
  (bind _asmy_character (cast `/Game/Core/MyCharacter` (`GameplayStatics.GetPlayerCharacter` 0)))
  (`/Engine/EditorBlueprintResources/StandardMacros.IsValid` _asmy_character
    (:`Is Valid`
      (if (>= (`self.GetDistanceTo` _asmy_character self) (`self.DistanceMaxFromPlayer`))
        (`KismetSystemLibrary.K2_ClearAndInvalidateTimerHandle` (`self.Timer`) :!label _label)
        (`self.K2_DestroyActor`)))
    (:`Is Not Valid`
      (goto _label))))

(event `self.Box.OnComponentBeginOverlap`
  (params (OverlappedComponent :type "PrimitiveComponent Object Reference") (OtherActor :type "Actor Object Reference") (OtherComp :type "PrimitiveComponent Object Reference") (OtherBodyIndex :type Integer) (bFromSweep :type Boolean) (SweepResult :type "HitResult Structure (by ref)"))
  ;[1 1 1 1 100] Gestion des degats au joueur
  ;;[1 1 1] Degats repetesAuJoueur
  (set `self.PlayerInRange` true)
  (bind _asmy_character (cast `/Game/Core/MyCharacter` OtherActor))
  (bind _output_get (set `self.As My Character` _asmy_character))
  (`/Engine/EditorBlueprintResources/StandardMacros.IsValid` _output_get
    (:`Is Valid`
      (`/Game/Core/MyCharacter.AffectHealth` _output_get (`self.DamageAmount`))
      (bind _returnvalue (`KismetSystemLibrary.K2_SetTimerDelegate` (delegate `DamageHero`) (/ 1.0 (`self.AttackPerSecond`)) true))
      (set `self.Timer` _returnvalue))
    (:`Is Not Valid`
      (set `self.PlayerInRange` false))))

(event `DamageHero`
  (bind _as_my_character (`self.As My Character`))
  ;[1 1 1 1 100] Gestion des degats au joueur
  ;;[1 1 1] Degats repetesAuJoueur
  ;;;[1 1 1] DegatsAuJoueur
  (if (`self.PlayerInRange`)
    (`/Engine/EditorBlueprintResources/StandardMacros.IsValid` _as_my_character
      (:`Is Valid`
        (`/Game/Core/BPInterfaces/BPI_Damageable.AffectHealth` _as_my_character (`self.DamageAmount`))))))

(event `self.Box.OnComponentEndOverlap`
  (params (OverlappedComponent :type "PrimitiveComponent Object Reference") (OtherActor :type "Actor Object Reference") (OtherComp :type "PrimitiveComponent Object Reference") (OtherBodyIndex :type Integer))
  ;[1 1 1 1 100] Gestion des degats au joueur
  ;;[1 1 1] Arret des degats au joueur
  (if (== OtherActor (`self.As My Character`))
    (`|ExecutionSequence`
      (:`then_0`
        (set `self.PlayerInRange` false)
        (`KismetSystemLibrary.K2_ClearAndInvalidateTimerHandle` (`self.Timer`))))))

(event `self.SaphirInteraction`
  (params (Delta :type "Float (single-precision)") (interactor :type "Actor Object Reference"))
  ;[1 1 1 1 150] DegatsRecus
  ;;[1 1 1] SimpleGunDamages
  (`self.UpdateHealthPoints` -1.0)
  (if (`self.IsDead`)
    (if (<= (`self.LootHealFloat`) (`KismetMathLibrary.RandomFloatInRange` 0.0 100.0))
      (`|SpawnActorFromClass` "/Game/Core/LootableItems/BP_HealthItem.BP_HealthItem_C" (`KismetMathLibrary.Conv_VectorToTransform` (`SceneComponent.K2_GetComponentLocation` (`self.CapsuleComponent`))) "Undefined" "OverrideRootScale" null null))
    (if (<= (`self.LootSaphir`) (`KismetMathLibrary.RandomFloatInRange` 0.0 100.0))
      (`|SpawnActorFromClass` "/Game/Core/LootableItems/BP_SaphirItem.BP_SaphirItem_C" (`KismetMathLibrary.Conv_VectorToTransform` (`SceneComponent.K2_GetComponentLocation` (`self.CapsuleComponent`))) "Undefined" "OverrideRootScale" null null))
    (`self.K2_DestroyActor`)))

(event `self.Capsule.OnComponentBeginOverlap`
  (params (OverlappedComponent :type "PrimitiveComponent Object Reference") (OtherActor :type "Actor Object Reference") (OtherComp :type "PrimitiveComponent Object Reference") (OtherBodyIndex :type Integer) (bFromSweep :type Boolean) (SweepResult :type "HitResult Structure (by ref)"))
  (if (== OtherActor (`self.LasrSaphir`))
    (`self.SaphirInteraction` 0.0)
    (`KismetSystemLibrary.PrintString` "Hello")
    (else
      (`self.SaphirStop`)
      (`KismetSystemLibrary.PrintString` "good"))))

(fn `DiamantDamages`
  (params (DeltaDiamant :type "Float (double-precision)" :default -1.0))
  (returns (NewHealth :type "Float (double-precision)"))
  (bind _output_get (set `self.Health` (+ (`self.Health`) DeltaDiamant)))
  (`self.UpdateIsDead`)
  (return _output_get))

(fn `EmeraudeDamages`
  (params (DeltaEmeraude :type "Float (double-precision)" :default -1.0))
  (returns (NewHealth :type "Float (double-precision)"))
  (bind _output_get (set `self.Health` (+ (`self.Health`) DeltaEmeraude)))
  (`self.UpdateIsDead`)
  (return _output_get))

(fn `RubisDamages`
  (params (DeltaRubis :type "Float (double-precision)" :default -1.0))
  (returns (NewHealth :type "Float (double-precision)"))
  (bind _output_get (set `self.Health` (+ (`self.Health`) DeltaRubis)))
  (`self.UpdateIsDead`)
  (return _output_get))

(fn `SaphirDamages`
  (params (DeltaSaphir :type "Float (double-precision)" :default 0.0))
  (returns (NewHealth :type "Float (double-precision)"))
  (bind _output_get (set `self.Health` (+ (`self.Health`) DeltaSaphir)))
  (`self.UpdateIsDead`)
  (return _output_get))

(fn `UpdateHealthPoints`
  (params (Delta :type "Float (double-precision)" :default -1.0))
  (returns (NewHealth :type "Float (double-precision)"))
  (bind _output_get (set `self.Health` (+ (`self.Health`) Delta)))
  (`self.UpdateIsDead`)
  (return _output_get))

(fn `UpdateIsDead`
  (if (<= (`self.Health`) 0.0)
    (set `self.IsDead` true)
    (`KismetSystemLibrary.K2_PauseTimer` null "UpdateHealthPoints")
    (else
      (set `self.IsDead` false))))

(fn `UserConstructionScript`)