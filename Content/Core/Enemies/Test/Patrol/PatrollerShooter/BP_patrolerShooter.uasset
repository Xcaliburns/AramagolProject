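; Patrolling shooter enemy Blueprint that fires projectiles, takes health changes and dies at zero health.
; EnemyShot spawns a basic enemy projectile at its arrow, while AffectHealth updates and prints Health, setting IsDead.
; On death, a random roll against LootHealFloat may spawn a health item and show a door-opened widget.
; Both outcomes invert the Interaction message and destroy the actor immediately, without waiting for the widget's removal delay.
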(event `EnemyShot`
  (`|SpawnActorFromClass` "/Game/Core/WeaponsAndProjectiles/BP_ProjectileBasicEnemy.BP_ProjectileBasicEnemy_C" (`SceneComponent.K2_GetComponentToWorld` (`self.Arrow1`)) "Undefined" "OverrideRootScale" null null))

(event `/Game/Core/BPInterfaces/BPI_Damageable.AffectHealth`
  (params (Delta :type "Float (single-precision)"))
  ;[1 1 1] Gestion des degats Self
  (bind _newhealth (`self.UpdateHealthPoints` Delta))
  (`KismetSystemLibrary.PrintString` (`KismetStringLibrary.Conv_DoubleToString` _newhealth))
  (if (`self.IsDead`)
    ;[1 1 1] Loot
    (if (<= (`self.LootHealFloat`) (`KismetMathLibrary.RandomFloatInRange` 0.0 100.0))
      (`|SpawnActorFromClass` "/Game/Core/LootableItems/BP_HealthItem.BP_HealthItem_C" (`KismetMathLibrary.Conv_VectorToTransform` (`SceneComponent.K2_GetComponentLocation` (`self.CapsuleComponent`))) "Undefined" "OverrideRootScale" null null)
      (`|ExecutionSequence`
        (:`then_0`
          (bind _returnvalue (`|CreateWidget` "/Game/Core/WBP/WBP_DoorOpened.WBP_DoorOpened_C"))
          (`UserWidget.AddToViewport` _returnvalue 0)
          (`KismetSystemLibrary.Delay` 5.0)
          (`Widget.RemoveFromParent` _returnvalue))
        (:`then_1`
          (message `/Game/Core/BPInterfaces/BPI_InverseInteract.Inverse` (`self.Interaction`) null :!label _label)
          (`self.K2_DestroyActor`)))
      (else
        (goto _label)))))

(fn `UpdateHealthPoints`
  (params (Delta :type "Float (double-precision)"))
  (returns (NewHealth :type "Float (double-precision)"))
  (bind _output_get (set `self.Health` (+ (`self.Health`) Delta)))
  (`self.UpdateIsDead`)
  (return _output_get))

(fn `UpdateIsDead`
  (if (<= (`self.Health`) 0.0)
    (set `self.IsDead` true)
    (`KismetSystemLibrary.K2_PauseTimer` null "UpdateHealthPoints")
    (else
      (set `self.IsDead` false))))

(fn `UserConstructionScript`)