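; Melee patroller enemy that damages the player on contact and can drop a health item when killed; no patrol logic appears here.
; Box overlap casts to MyCharacter, hits immediately, then repeats through a looping timer at AttackPerSecond until that character exits.
; AffectHealth adds a delta to Health and updates IsDead.
; On death, it spawns BP_HealthItem if a 0–100 roll reaches at least LootHealFloat, then destroys itself.
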(event `self.Box.OnComponentBeginOverlap`
  (params (OverlappedComponent :type "PrimitiveComponent Object Reference") (OtherActor :type "Actor Object Reference") (OtherComp :type "PrimitiveComponent Object Reference") (OtherBodyIndex :type Integer) (bFromSweep :type Boolean) (SweepResult :type "HitResult Structure (by ref)"))
  ;[1 1 1] Gestion des degats au joueur
  ;;[1 1 1] Degats repetesAuJoueur
  (set `self.PlayerInRange` true)
  (bind _asmy_character (cast `/Game/Core/MyCharacter` OtherActor))
  (bind _output_get (set `self.As My Character` _asmy_character))
  (`/Engine/EditorBlueprintResources/StandardMacros.IsValid` _output_get
    (:`Is Valid`
      (`/Game/Core/MyCharacter.AffectHealth` _output_get (`self.DamageAmount`))
      (bind _returnvalue (`KismetSystemLibrary.K2_SetTimerDelegate` (delegate `DamageHero`) (/ 1.0 (`self.AttackPerSecond`)) true))
      (set `self.Timer` _returnvalue))
    (:`Is Not Valid`
      (set `self.PlayerInRange` false))))

(event `DamageHero`
  (bind _as_my_character (`self.As My Character`))
  ;[1 1 1] Gestion des degats au joueur
  ;;[1 1 1] Degats repetesAuJoueur
  ;;;[1 1 1] DegatsAuJoueur
  (if (`self.PlayerInRange`)
    (`/Engine/EditorBlueprintResources/StandardMacros.IsValid` _as_my_character
      (:`Is Valid`
        (`/Game/Core/BPInterfaces/BPI_Damageable.AffectHealth` _as_my_character (`self.DamageAmount`))))))

(event `self.Box.OnComponentEndOverlap`
  (params (OverlappedComponent :type "PrimitiveComponent Object Reference") (OtherActor :type "Actor Object Reference") (OtherComp :type "PrimitiveComponent Object Reference") (OtherBodyIndex :type Integer))
  ;[1 1 1] Gestion des degats au joueur
  ;;[1 1 1] Arret des degats au joueur
  (if (== OtherActor (`self.As My Character`))
    (`|ExecutionSequence`
      (:`then_0`
        (set `self.PlayerInRange` false)
        (`KismetSystemLibrary.K2_ClearAndInvalidateTimerHandle` (`self.Timer`))))))

(event `/Game/Core/BPInterfaces/BPI_Damageable.AffectHealth`
  (params (Delta :type "Float (single-precision)"))
  ;[1 1 1] Gestion des degats Self
  (`self.UpdateHealthPoints` Delta)
  (if (`self.IsDead`)
    ;[1 1 1] Loot
    (if (<= (`self.LootHealFloat`) (`KismetMathLibrary.RandomFloatInRange` 0.0 100.0))
      (`|SpawnActorFromClass` "/Game/Core/LootableItems/BP_HealthItem.BP_HealthItem_C" (`KismetMathLibrary.Conv_VectorToTransform` (`SceneComponent.K2_GetComponentLocation` (`self.CapsuleComponent`))) "Undefined" "OverrideRootScale" null null))
    (`self.K2_DestroyActor`)))

(fn `UpdateHealthPoints`
  (params (Delta :type "Float (double-precision)"))
  (returns (NewHealth :type "Float (double-precision)"))
  (bind _output_get (set `self.Health` (+ (`self.Health`) Delta)))
  (`self.UpdateIsDead`)
  (return _output_get))

(fn `UpdateIsDead`
  (if (<= (`self.Health`) 0.0)
    (set `self.IsDead` true)
    (`KismetSystemLibrary.K2_PauseTimer` null "UpdateHealthPoints")
    (else
      (set `self.IsDead` false))))

(fn `UserConstructionScript`)