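; BP_Boss001 is a test boss enemy with laser and projectile attacks, health tracking and a health-item drop.
; LaserStartSaphir attaches a spawned laser to a spine socket behind a delay-based cooldown, while EnemyShot fires projectiles from an arrow.
; AffectHealth updates health and death state; only a successful loot roll on death spawns the item, then messages Interactors and destroys the boss inside that loop.
; The construction script applies five mesh materials.
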(event `self.ReceiveBeginPlay`
  (set `self.LaserReady` true))

(event `LaserStartSaphir`
  (bind _mesh (`self.Mesh`))
  (bind (_returnvalue_location _returnvalue_rotation _returnvalue_scale) (`KismetMathLibrary.BreakTransform` (`SceneComponent.K2_GetComponentToWorld` _mesh)))
  (if (`self.LaserReady`)
    (set `self.LaserReady` false)
    (bind _returnvalue (`|SpawnActorFromClass` "/Game/Core/WeaponsAndProjectiles/BP_LaserEnemy.BP_LaserEnemy_C" (`KismetMathLibrary.MakeTransform` _returnvalue_location _returnvalue_rotation (/ _returnvalue_scale 10)) "Undefined" "OverrideRootScale" null null))
    (`self.K2_AttachToComponent` _returnvalue _mesh "spine_004Socket" "SnapToTarget" "SnapToTarget" "SnapToTarget" true)
    (`KismetSystemLibrary.Delay` 2.3)
    (set `self.LaserReady` true)))

(event `EnemyShot`
  (`|SpawnActorFromClass` "/Game/Core/WeaponsAndProjectiles/BP_ProjectileBasicEnemy.BP_ProjectileBasicEnemy_C" (`SceneComponent.K2_GetComponentToWorld` (`self.Arrow1`)) "Undefined" "OverrideRootScale" null null))

(event `/Game/Core/BPInterfaces/BPI_Damageable.AffectHealth`
  (params (Delta :type "Float (single-precision)"))
  (bind _interactor (`self.Interactor`))
  ;[1 1 1] Gestion des degats Self
  (bind _newhealth (`self.UpdateHealthPoints` Delta))
  (`KismetSystemLibrary.PrintString` (`KismetStringLibrary.Conv_DoubleToString` _newhealth))
  (if (`self.IsDead`)
    ;[1 1 1] Loot
    (if (<= (`self.LootHealFloat`) (`KismetMathLibrary.RandomFloatInRange` 0.0 100.0))
      (`|SpawnActorFromClass` "/Game/Core/LootableItems/BP_HealthItem.BP_HealthItem_C" (`KismetMathLibrary.Conv_VectorToTransform` (`SceneComponent.K2_GetComponentLocation` (`self.CapsuleComponent`))) "Undefined" "OverrideRootScale" null null)
      (for (_ _array_index) _interactor
        (message `/Game/Core/BPInterfaces/BPI_InverseInteract.Inverse` (`|GetArrayItem` _interactor _array_index) null)
        (`self.K2_DestroyActor`)))))

(fn `UpdateHealthPoints`
  (params (Delta :type "Float (double-precision)"))
  (returns (NewHealth :type "Float (double-precision)"))
  (bind _output_get (set `self.Health` (+ (`self.Health`) Delta)))
  (`self.UpdateIsDead`)
  (return _output_get))

(fn `UpdateIsDead`
  (if (<= (`self.Health`) 0.0)
    (set `self.IsDead` true)
    (else
      (set `self.IsDead` false))))

(fn `UserConstructionScript`
  (bind _mesh (`self.Mesh`))
  (`PrimitiveComponent.SetMaterial` _mesh 0 (`self.Material0`))
  (`PrimitiveComponent.SetMaterial` _mesh 1 (`self.Material1`))
  (`PrimitiveComponent.SetMaterial` _mesh 2 (`self.Material2`))
  (`PrimitiveComponent.SetMaterial` _mesh 3 (`self.Material3`))
  (`PrimitiveComponent.SetMaterial` _mesh 4 (`self.Material4`)))