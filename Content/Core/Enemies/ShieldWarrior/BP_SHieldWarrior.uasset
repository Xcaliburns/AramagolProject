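; BP_SHieldWarrior is an enemy that fires BP_ProjectileBasicEnemy from an arrow component on a looping timer started at BeginPlay.
; AffectHealth adds a delta to Health and updates IsDead, briefly swapping to a flash material if the enemy survives.
; On death it destroys itself; a random roll against Loot gates the crystal drop, camera shake and Niagara destruction effect together.
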(event `self.ReceiveBeginPlay`
  (`self.ShotTimer`))

(event `ShotTimer`
  (`KismetSystemLibrary.K2_SetTimerDelegate` (delegate `Shot`) 1.0 true 2.0))

(event `Shot`
  (`|SpawnActorFromClass` "/Game/Core/WeaponsAndProjectiles/BP_ProjectileBasicEnemy.BP_ProjectileBasicEnemy_C" (`SceneComponent.K2_GetComponentToWorld` (`self.Arrow1`)) "Undefined" "OverrideRootScale" null null))

(event `/Game/Core/BPInterfaces/BPI_Damageable.AffectHealth`
  (params (Delta :type "Float (single-precision)"))
  (bind _mesh (`self.Mesh`))
  (bind _returnvalue (`SceneComponent.K2_GetComponentLocation` (`self.CapsuleComponent`)))
  (`self.UpdateHealthPoints` Delta)
  (if (`self.IsDead`)
    (if (<= (`self.Loot`) (`KismetMathLibrary.RandomFloatInRange` 0.0 100.0))
      (`|SpawnActorFromClass` "/Game/Core/LootableItems/BP_CoarseCristal.BP_CoarseCristal_C" (`KismetMathLibrary.Conv_VectorToTransform` _returnvalue) "Undefined" "OverrideRootScale" null null)
      (`GameplayStatics.PlayWorldCameraShake` "/Game/Core/Components/CS_CommonEnemyDestroyed.CS_CommonEnemyDestroyed_C" (`self.K2_GetActorLocation`) 0.0 2500.0)
      (`NiagaraFunctionLibrary.SpawnSystemAtLocation` "/Game/Core/FX/destroyedEnemy/NS_Destroy.NS_Destroy" _returnvalue))
    (`self.K2_DestroyActor`)
    (else
      (`PrimitiveComponent.SetMaterial` _mesh 0 "/Game/Core/Material/MI_Flash.MI_Flash")
      (`KismetSystemLibrary.Delay` 0.1)
      (`PrimitiveComponent.SetMaterial` _mesh 0 "/Game/Core/Enemies/Miniboss001Materials/Blue.Blue"))))

(fn `UpdateHealthPoints`
  (params (Delta :type "Float (double-precision)" :default -1.0))
  (returns (NewHealth :type "Float (double-precision)"))
  (bind _output_get (set `self.Health` (+ (`self.Health`) Delta)))
  (`KismetSystemLibrary.PrintString` (`KismetStringLibrary.Conv_DoubleToString` _output_get))
  (`self.UpdateIsDead`)
  (return _output_get))

(fn `UpdateIsDead`
  (if (<= (`self.Health`) 0.0)
    (set `self.IsDead` true)
    (`KismetSystemLibrary.K2_PauseTimer` null "UpdateHealthPoints")
    (else
      (set `self.IsDead` false))))

(fn `UserConstructionScript`)