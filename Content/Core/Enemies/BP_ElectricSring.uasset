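; BP_ElectricSring is an electric hazard that damages the player character while it overlaps the Collision component.
; Begin overlap casts to MyCharacter, applies a negative AffectHealth hit at once, then starts a looping half-second timer that repeats the damage on the stored character.
; End overlap pauses that timer when the leaving actor has the Player tag.
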(event `TimerDamage`
  (bind _returnvalue (`KismetSystemLibrary.K2_SetTimerDelegate` (delegate `Damages`) 0.5 true))
  (set `self.TimerDamageHandle` _returnvalue))

(event `Damages`
  (`/Game/Core/MyCharacter.AffectHealth` (`self.As My Character`) -25.0))

(event `self.Collision.OnComponentBeginOverlap`
  (params (OverlappedComponent :type "PrimitiveComponent Object Reference") (OtherActor :type "Actor Object Reference") (OtherComp :type "PrimitiveComponent Object Reference") (OtherBodyIndex :type Integer) (bFromSweep :type Boolean) (SweepResult :type "HitResult Structure (by ref)"))
  (bind _asmy_character (cast `/Game/Core/MyCharacter` OtherActor))
  (bind _output_get (set `self.As My Character` _asmy_character))
  (`/Game/Core/MyCharacter.AffectHealth` _output_get -25.0)
  (`self.TimerDamage`))

(event `self.Collision.OnComponentEndOverlap`
  (params (OverlappedComponent :type "PrimitiveComponent Object Reference") (OtherActor :type "Actor Object Reference") (OtherComp :type "PrimitiveComponent Object Reference") (OtherBodyIndex :type Integer))
  (if (`self.ActorHasTag` OtherActor "Player")
    (`KismetSystemLibrary.K2_PauseTimerHandle` (`self.TimerDamageHandle`))))

(fn `UserConstructionScript`)