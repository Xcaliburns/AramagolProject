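; BP_Teleporteur3Cristaux is a teleporter that stays inactive until its three crystals (Rubis, Emeraude, Saphir) have all been activated.
; Each crystal's interaction event sets its flag, then a shared check reveals the Sphere component once all three are true.
; When a MyCharacter overlaps the Box with all flags set, player 0's character teleports to the Destination actor's location and rotation.
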(event `self.Box.OnComponentBeginOverlap`
  (params (OverlappedComponent :type "PrimitiveComponent Object Reference") (OtherActor :type "Actor Object Reference") (OtherComp :type "PrimitiveComponent Object Reference") (OtherBodyIndex :type Integer) (bFromSweep :type Boolean) (SweepResult :type "HitResult Structure (by ref)"))
  (bind (_returnvalue_location _returnvalue_rotation) (`KismetMathLibrary.BreakTransform` (`self.GetTransform` (`self.Destination`))))
  (cast `/Game/Core/MyCharacter` OtherActor)
  (if (and (`self.Emeraude`) (`self.saphir`) (`self.Rubis`))
    (`self.K2_TeleportTo` (`GameplayStatics.GetPlayerCharacter` 0) _returnvalue_location _returnvalue_rotation)))

(event `/Game/Core/BPInterfaces/BPI_RubisInteract.RubisInteraction`
  (set `self.Rubis` true)
  (if (and (`self.Emeraude`) (`self.saphir`) (`self.Rubis`)) :!label _label
    (`SceneComponent.SetVisibility` (`self.Sphere`) true false)))

(event `/Game/Core/BPInterfaces/BPI_EmeraudeInteract.EmeraudeInteraction`
  (set `self.Emeraude` true)
  (goto _label))

(event `/Game/Core/BPInterfaces/BPI_SaphirInteract.SaphirInteraction`
  (params (Delta :type "Float (single-precision)") (interactor :type "Actor Object Reference"))
  (set `self.saphir` true)
  (goto _label))

(fn `UserConstructionScript`)