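; Double door to the deep jungle that swings open when the player enters its trigger or when it receives an Interactable event.
; The MoveDoor timeline drives the yaw of both leaves, with each track feeding the oppositely named leaf.
; Trigger openings reverse the timeline after a three-second delay and print a debug string, while Interactable openings have no automatic close.
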(event `/Game/Core/BPInterfaces/BPI_Interactable.Interactable`
  (params (Interactor :type "Actor Object Reference"))
  (`self.OpenDoor`))

(event `self.Trigger.OnComponentBeginOverlap`
  (params (OverlappedComponent :type "PrimitiveComponent Object Reference") (OtherActor :type "Actor Object Reference") (OtherComp :type "PrimitiveComponent Object Reference") (OtherBodyIndex :type Integer) (bFromSweep :type Boolean) (SweepResult :type "HitResult Structure (by ref)"))
  (if (`self.ActorHasTag` OtherActor "Player")
    (`self.OpenDoor`)
    (`KismetSystemLibrary.Delay` 3.0)
    (`self.CloseDoor`)))

(event `self.Trigger.OnComponentEndOverlap`
  (params (OverlappedComponent :type "PrimitiveComponent Object Reference") (OtherActor :type "Actor Object Reference") (OtherComp :type "PrimitiveComponent Object Reference") (OtherBodyIndex :type Integer)))

(event `OpenDoor`
  (bind (_direction _battantdroit _battantgauche) (`Timeline|MoveDoor` :!label _label)
    (:`Update`
      (`SceneComponent.K2_SetRelativeRotation` (`self.BattantDroit`) (`KismetMathLibrary.MakeRotator` 0.0 0.0 _battantgauche) false false)
      (`SceneComponent.K2_SetRelativeRotation` (`self.BattantGauche`) (`KismetMathLibrary.MakeRotator` 0.0 0.0 _battantdroit) false false))))

(event `CloseDoor`
  (`KismetSystemLibrary.PrintString` "Hello")
  (goto _label :!via `Reverse`))

(fn `UserConstructionScript`)