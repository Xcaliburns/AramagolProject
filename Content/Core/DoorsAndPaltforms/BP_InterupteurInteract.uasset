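; BP_InterupteurInteract is a trigger switch that fires when an actor tagged Player overlaps its Box.
; Each overlap sends InteractableMessage to every entry in the Interactor array, so one switch can drive several targets.
; A DoOnce then shows the WBP_DoorOpened widget on the first trigger only and removes it after a short delay.
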(event `self.Box.OnComponentBeginOverlap`
  (params (OverlappedComponent :type "PrimitiveComponent Object Reference") (OtherActor :type "Actor Object Reference") (OtherComp :type "PrimitiveComponent Object Reference") (OtherBodyIndex :type Integer) (bFromSweep :type Boolean) (SweepResult :type "HitResult Structure (by ref)"))
  (bind _interactor (`self.Interactor`))
  (if (`self.ActorHasTag` OtherActor "Player")
    (`|ExecutionSequence`
      (:`then_0`
        (for (_ _array_index) _interactor
          (message `/Game/Core/BPInterfaces/BPI_Interactable.Interactable` (`|GetArrayItem` _interactor _array_index) null)))
      (:`then_1`
        (`/Engine/EditorBlueprintResources/StandardMacros.DoOnce` false
          (:`Completed`
            (bind _returnvalue (`|CreateWidget` "/Game/Core/WBP/WBP_DoorOpened.WBP_DoorOpened_C"))
            (`UserWidget.AddToViewport` _returnvalue 0)
            (`KismetSystemLibrary.Delay` 5.0)
            (`Widget.RemoveFromParent` _returnvalue)))))))

(fn `UserConstructionScript`)