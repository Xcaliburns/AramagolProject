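; BP_InterrupteurParent is a parent switch Blueprint that triggers linked interactors once, when an actor overlaps its Box.
; The first valid overlap turns the Interrupteur green and spawns an attached DirectionalBurst effect.
; It then calls InverseMessage on every entry in the Interactor array and shows the WBP_DoorOpened widget for a few seconds before removing it.
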(event `self.Box.OnComponentBeginOverlap`
  (params (OverlappedComponent :type "PrimitiveComponent Object Reference") (OtherActor :type "Actor Object Reference") (OtherComp :type "PrimitiveComponent Object Reference") (OtherBodyIndex :type Integer) (bFromSweep :type Boolean) (SweepResult :type "HitResult Structure (by ref)"))
  (bind _interrupteur (`self.Interrupteur`))
  (bind _interactor (`self.Interactor`))
  (`/Engine/EditorBlueprintResources/StandardMacros.IsValid` OtherActor
    (:`Is Valid`
      (`/Engine/EditorBlueprintResources/StandardMacros.DoOnce` false
        (:`Completed`
          (`PrimitiveComponent.SetMaterial` _interrupteur 1 "/Game/Core/Starships/vert.vert")
          (`NiagaraFunctionLibrary.SpawnSystemAttached` "/Niagara/DefaultAssets/Templates/Systems/DirectionalBurst.DirectionalBurst" _interrupteur "None" (0.0 0.0 0.0) (struct) "KeepRelativeOffset")
          (`|ExecutionSequence`
            (:`then_0`
              (for (_ _array_index) _interactor
                (message `/Game/Core/BPInterfaces/BPI_InverseInteract.Inverse` (`|GetArrayItem` _interactor _array_index) null)))
            (:`then_1`
              (bind _returnvalue (`|CreateWidget` "/Game/Core/WBP/WBP_DoorOpened.WBP_DoorOpened_C"))
              (`UserWidget.AddToViewport` _returnvalue 0)
              (`KismetSystemLibrary.Delay` 5.0)
              (`Widget.RemoveFromParent` _returnvalue))))))))

(fn `UserConstructionScript`)