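; BP_Teleporteur is a teleporter that sends the player character to a destination actor, gated by the sapphire key (CleSaphir).
; When MyCharacter overlaps its Box and has that flag set, it plays the character's teleport effect, waits briefly, then moves it to the Destination's location and rotation.
; After a further short delay it calls Respawn on the character.
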(event `self.Box.OnComponentBeginOverlap`
  (params (OverlappedComponent :type "PrimitiveComponent Object Reference") (OtherActor :type "Actor Object Reference") (OtherComp :type "PrimitiveComponent Object Reference") (OtherBodyIndex :type Integer) (bFromSweep :type Boolean) (SweepResult :type "HitResult Structure (by ref)"))
  (bind (_returnvalue_location _returnvalue_rotation) (`KismetMathLibrary.BreakTransform` (`self.GetTransform` (`self.Destination`))))
  (bind _asmy_character (cast `/Game/Core/MyCharacter` OtherActor))
  (if (`/Game/Core/MyCharacter.CleSaphir` _asmy_character)
    (`|ExecutionSequence`
      (:`then_0`
        (`/Game/Core/MyCharacter.Teleport Effect` _asmy_character)
        (`KismetSystemLibrary.Delay` 2.0)
        (`self.K2_TeleportTo` _asmy_character _returnvalue_location _returnvalue_rotation)
        (`KismetSystemLibrary.Delay` 0.2)
        (`/Game/Core/MyCharacter.Respawn` _asmy_character)))))

(fn `UserConstructionScript`)